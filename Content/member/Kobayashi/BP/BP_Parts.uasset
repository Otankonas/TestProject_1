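; BP_Parts is a parts Blueprint that applies shared materials to a set of ten left and right "Ita" components.
; The construction script passes the components to SetTarget, which loops over the Target array and appends one to it per index through a switch.
; SetMaterial then assigns the first two Material array entries to slots 0 and 1 of each target.
; The event graph holds only disabled default events.
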(fn `SetMaterial`
  (params (`Dimension 1` :type Integer))
  (bind _output (`|GetArrayItem` (`self.Target`) `Dimension 1`))
  (`PrimitiveComponent.SetMaterial` _output 0 (`|GetArrayItem` (`self.Material`)))
  (`PrimitiveComponent.SetMaterial` _output 1 (`|GetArrayItem` (`self.Material`) 1)))

(fn `SetTarget`
  (params (NewParam1 :type "StaticMeshComponent Object Reference") (NewParam2 :type "StaticMeshComponent Object Reference") (NewParam3 :type "StaticMeshComponent Object Reference") (NewParam4 :type "StaticMeshComponent Object Reference") (NewParam5 :type "StaticMeshComponent Object Reference") (NewParam6 :type "StaticMeshComponent Object Reference") (NewParam7 :type "StaticMeshComponent Object Reference") (NewParam8 :type "StaticMeshComponent Object Reference") (NewParam9 :type "StaticMeshComponent Object Reference") (NewParam10 :type "StaticMeshComponent Object Reference"))
  (bind _target (`self.Target`))
  (for (_ _array_index) (`self.Target`)
    (switch `int` _array_index
      (:`0`
        (`KismetArrayLibrary.Array_Add` _target NewParam1))
      (:`1`
        (`KismetArrayLibrary.Array_Add` _target NewParam2))
      (:`2`
        (`KismetArrayLibrary.Array_Add` _target NewParam3))
      (:`3`
        (`KismetArrayLibrary.Array_Add` _target NewParam4))
      (:`4`
        (`KismetArrayLibrary.Array_Add` _target NewParam5))
      (:`5`
        (`KismetArrayLibrary.Array_Add` _target NewParam6))
      (:`6`
        (`KismetArrayLibrary.Array_Add` _target NewParam7))
      (:`7`
        (`KismetArrayLibrary.Array_Add` _target NewParam8))
      (:`8`
        (`KismetArrayLibrary.Array_Add` _target NewParam9))
      (:`9`
        (`KismetArrayLibrary.Array_Add` _target NewParam10)))))

(fn `UserConstructionScript`
  (`self.SetTarget` (`self.GP00_K_L_ita_3`) (`self.GP00_K_L_ita_2`) (`self.GP00_K_L_ita_1`) (`self.GP00_K_R_ita_S_1`) (`self.GP00_K_R_ita_S_2`) (`self.GP00_K_R_ita_3`) (`self.GP00_K_R_ita_2`) (`self.GP00_K_R_ita_1`) (`self.GP00_K_L_ita_S_1`) (`self.GP00_K_L_ita_S_2`))
  (for (_ _array_index) (`self.Target`)
    (`self.SetMaterial` _array_index)))