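; BP_Bhooooon1 is an actor that follows the player's BP_PlayerBaseV4 mesh; its wider purpose is not shown.
; BeginPlay casts and caches player pawn 0, then runs the same snap step that Tick repeats.
; That step moves the actor to the mesh's world location and applies the mesh's relative rotation as the root's world rotation.
; NewMacro holds only an unused angle calculation.
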(event `self.ReceiveBeginPlay`
  (bind _mesh (`Character.Mesh` (`self.As BP Player Base V4`)))
  (bind _asbp_player_base_v4 (cast `/Game/member/Okajima/PlayerSource/BP_PlayerBaseV4` (`GameplayStatics.GetPlayerPawn` 0)))
  (set `self.As BP Player Base V4` _asbp_player_base_v4)
  (`self.K2_SetActorLocation` self (`SceneComponent.K2_GetComponentLocation` _mesh) false false :!label _label)
  (`SceneComponent.K2_SetWorldRotation` (`self.DefaultSceneRoot`) (`SceneComponent.RelativeRotation` _mesh) false false))

(event `self.ReceiveTick`
  (params (DeltaSeconds :type "Float (single-precision)"))
  (goto _label))

(fn `UserConstructionScript`)