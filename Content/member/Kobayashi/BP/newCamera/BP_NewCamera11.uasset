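; BP_NewCamera11 is a camera Blueprint that makes itself player 0's view target on BeginPlay.
; It caches the player pawn's location once at startup and calls SetActorLocation every Tick, with no new location supplied.
; A SetLocation function repeats that bare call, and an unconnected Lerp on the cached Y suggests unfinished smoothing.
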(event `self.ReceiveBeginPlay`
  (`PlayerController.SetViewTargetWithBlend` (`GameplayStatics.GetPlayerController` 0) self 0.0 "VTBlend_Linear" 0.0 false)
  (set `self.PlayerLocation` (`self.K2_GetActorLocation` (`GameplayStatics.GetPlayerPawn` 0))))

(event `self.ReceiveTick`
  (params (DeltaSeconds :type "Float (single-precision)"))
  (`self.K2_SetActorLocation` (0.0 0.0 0.0)))

(fn `SetLocation`
  (params (deltaTime :type "Float (double-precision)") (PlayerLocation :type "Vector Structure") (CameraLocation :type "Vector Structure"))
  (`self.K2_SetActorLocation` (0.0 0.0 0.0)))

(fn `UserConstructionScript`)