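; First-person camera actor that follows the player pawn's capsule with a height offset, matches its rotation and can become the view target.
; Tick updates the follow transform and caches it while UseCamera3 is set.
; ToCamera2 and ToCamera4 events pause following, then use timelines to interpolate from the cached transform to the other camera.
; On finish they trigger that camera's third-person event and resume following; the Camera2 reference is not assigned here.
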(event `self.ReceiveBeginPlay`
  (bind _as_bp_player_base_v4 (`self.As BP Player Base V4`))
  (bind (_returnvalue_x _returnvalue_y _returnvalue_z) (`KismetMathLibrary.BreakVector` (`SceneComponent.K2_GetComponentLocation` (`Character.CapsuleComponent` _as_bp_player_base_v4))))
  (bind _asbp_player_base_v4 (cast `/Game/member/Okajima/PlayerSource/BP_PlayerBaseV4` (`GameplayStatics.GetPlayerPawn` 0)))
  (set `self.As BP Player Base V4` _asbp_player_base_v4)
  (bind _returnvalue (`GameplayStatics.GetActorOfClass` "/Game/member/Kobayashi/BP/newCamera/BP_NewCamera4.BP_NewCamera4_C"))
  (set `self.As BP NewCamera4` _returnvalue)
  (`self.K2_SetActorLocationAndRotation` (`KismetMathLibrary.MakeVector` _returnvalue_x _returnvalue_y (+ _returnvalue_z 70.0)) (`self.K2_GetActorRotation` _as_bp_player_base_v4)))

(event `SetFirstPerson_Event`
  ;[1 1 1] カメラ切り替え
  (`PlayerController.SetViewTargetWithBlend` (`GameplayStatics.GetPlayerController` 0) self 0.0 "VTBlend_Linear" 0.0 false))

(event `ToCamera2_Event`
  (bind _keeplocation (`self.KeepLocation`))
  (bind (_keeprotation_roll _keeprotation_pitch _keeprotation_yaw) (`KismetMathLibrary.BreakRotator` (`self.KeepRotation`)))
  (bind _as_bp_newcamera2 (`self.As BP NewCamera2`))
  (bind (_returnvalue_roll _returnvalue_pitch _returnvalue_yaw) (`KismetMathLibrary.BreakRotator` (`self.K2_GetActorRotation` _as_bp_newcamera2)))
  ;[1 1 1] ToCamera2
  (set `self.UseCamera3` false)
  (bind (_direction _move) (`Timeline|タイムライン` :!via `PlayFromStart`)
    (:`Update`
      (`self.K2_SetActorLocationAndRotation` self (+ (* (- (`self.K2_GetActorLocation` _as_bp_newcamera2) _keeplocation) _move) _keeplocation) (`KismetMathLibrary.MakeRotator` (+ _keeprotation_roll (* (- _returnvalue_roll _keeprotation_roll) _move)) (+ _keeprotation_pitch (* (- _returnvalue_pitch _keeprotation_pitch) _move)) (+ _keeprotation_yaw (* (- _returnvalue_yaw _keeprotation_yaw) _move))) false false))
    (:`Finished`
      (`KismetSystemLibrary.PrintString` "完了")
      (`/Game/member/Kobayashi/BP/newCamera/BP_NewCamera2.SetThirdPerson_Event` _as_bp_newcamera2)
      (`self.K2_SetActorRotation` (`self.KeepRotation`))
      (set `self.UseCamera3` true))))

(event `self.ReceiveTick`
  (params (DeltaSeconds :type "Float (single-precision)"))
  (bind _as_bp_player_base_v4 (`self.As BP Player Base V4`))
  (bind (_returnvalue_x _returnvalue_y _returnvalue_z) (`KismetMathLibrary.BreakVector` (`SceneComponent.K2_GetComponentLocation` (`Character.CapsuleComponent` _as_bp_player_base_v4))))
  (if (`self.UseCamera3`)
    (`self.K2_SetActorLocationAndRotation` (`KismetMathLibrary.MakeVector` _returnvalue_x _returnvalue_y (+ _returnvalue_z 70.0)) (`self.K2_GetActorRotation` _as_bp_player_base_v4))
    (set `self.KeepLocation` (`self.K2_GetActorLocation`))
    (set `self.KeepRotation` (`self.K2_GetActorRotation`))))

(event `ToCamera4_Event`
  (bind _as_bp_newcamera4 (`self.As BP NewCamera4`))
  (bind _keeplocation (`self.KeepLocation`))
  (bind (_keeprotation_roll _keeprotation_pitch _keeprotation_yaw) (`KismetMathLibrary.BreakRotator` (`self.KeepRotation`)))
  (bind (_returnvalue_roll _returnvalue_pitch _returnvalue_yaw) (`KismetMathLibrary.BreakRotator` (`self.K2_GetActorRotation` _as_bp_newcamera4)))
  ;[1 1 1] ToCamera4
  (set `self.UseCamera3` false)
  (bind (_direction _move) (`Timeline|タイムライン_0` :!via `PlayFromStart`)
    (:`Update`
      (`self.K2_SetActorLocationAndRotation` self (+ (* (- (`self.K2_GetActorLocation` _as_bp_newcamera4) _keeplocation) _move) _keeplocation) (`KismetMathLibrary.MakeRotator` (+ _keeprotation_roll (* (- _returnvalue_roll _keeprotation_roll) _move)) (+ _keeprotation_pitch (* (- _returnvalue_pitch _keeprotation_pitch) _move)) (+ _keeprotation_yaw (* (- _returnvalue_yaw _keeprotation_yaw) _move))) false false))
    (:`Finished`
      (`KismetSystemLibrary.PrintString` "完了")
      (`/Game/member/Kobayashi/BP/newCamera/BP_NewCamera4.SetThirdPerson_Event` _as_bp_newcamera4)
      (`self.K2_SetActorRotation` (`self.KeepRotation`))
      (set `self.UseCamera3` true))))

(fn `UserConstructionScript`)