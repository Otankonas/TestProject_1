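; Follow camera actor that becomes the view target at BeginPlay, keeping a fixed X offset from the player's start.
; Each tick it tracks the pawn's Y, updates height only during jump moves, and eases spring arm length while attacking.
; ToCamera3_Event pauses following, rotates toward BP_NewCamera3 on a timeline, calls its first-person event, then restores its saved transform.
; The boss-room lerp is unconnected.
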(event `self.ReceiveBeginPlay`
  (bind _returnvalue (`GameplayStatics.GetPlayerController` 0))
  ;[1 1 1] 初期配置
  (`PlayerController.SetViewTargetWithBlend` _returnvalue self 0.0 "VTBlend_Linear" 0.0 false)
  (`self.SetLocationFirst` 400.0 (`self.K2_GetActorLocation` _returnvalue))
  (`self.K2_SetActorRotation` (`KismetMathLibrary.MakeRotator` 0.0))
  (bind _returnvalue_2 (`GameplayStatics.GetActorOfClass` "/Game/member/Kobayashi/BP/newCamera/BP_NewCamera3.BP_NewCamera3_C"))
  (set `self.AsBP_NewCamera3` _returnvalue_2))

(event `self.ReceiveTick`
  (params (DeltaSeconds :type "Float (single-precision)"))
  (bind _returnvalue (`self.K2_GetActorLocation` (`GameplayStatics.GetPlayerPawn` 0)))
  (if (`self.UseCamera2`)
    (if (`self.IsJumpMove`)
      (`self.SetLocation2D` _returnvalue)
      (else
        (`self.SetLocation` _returnvalue)))
    ;[1 1 1] カメラ距離調整
    (`self.CameraLengeLerp` (`self.IsAtack`) 0.1)
    (set `SpringArmComponent.TargetArmLength` (`KismetMathLibrary.Lerp` 0.0 -300.0 (`self.TargetLenLerp`)) (`self.SpringArm`))
    (set `self.KeepLocation` (`self.K2_GetActorLocation`))
    (set `self.KeepRotation` (`self.K2_GetActorRotation`))))

(event `SetThirdPerson_Event`
  ;[1 1 1] カメラ切り替え
  (`PlayerController.SetViewTargetWithBlend` (`GameplayStatics.GetPlayerController` 0) self 0.0 "VTBlend_Linear" 0.0 false))

(event `ToCamera3_Event`
  (bind (_keeprotation_roll _keeprotation_pitch _keeprotation_yaw) (`KismetMathLibrary.BreakRotator` (`self.KeepRotation`)))
  (bind _asbp_newcamera3 (`self.AsBP_NewCamera3`))
  (bind _keeplocation (`self.KeepLocation`))
  (bind (_returnvalue_roll _returnvalue_pitch _returnvalue_yaw) (`KismetMathLibrary.BreakRotator` (`self.K2_GetActorRotation` _asbp_newcamera3)))
  ;[1 1 1] カメラ切り替え
  (set `self.UseCamera2` false)
  (bind (_direction _move) (`Timeline|タイムライン` :!via `PlayFromStart`)
    (:`Update`
      (`self.K2_SetActorLocationAndRotation` self (+ (* (- (`self.K2_GetActorLocation`) _keeplocation) _move) _keeplocation) (`KismetMathLibrary.MakeRotator` (+ _keeprotation_roll (* (- _returnvalue_roll _keeprotation_roll) _move)) (+ _keeprotation_pitch (* (- _returnvalue_pitch _keeprotation_pitch) _move)) (+ _keeprotation_yaw (* (- _returnvalue_yaw _keeprotation_yaw) _move))) false false))
    (:`Finished`
      (`KismetSystemLibrary.PrintString` "完了")
      (`/Game/member/Kobayashi/BP/newCamera/BP_NewCamera3.SetFirstPerson_Event` _asbp_newcamera3)
      (`self.K2_SetActorLocationAndRotation` (`self.KeepLocation`) (`self.KeepRotation`))
      (set `self.UseCamera2` true))))

(fn `CameraLengeLerp`
  (params (IsAtack :type Boolean) (NewParam :type "Float (double-precision)"))
  (bind _targetlenlerp (`self.TargetLenLerp`))
  (if IsAtack
    (bind `_加算結果` (`self.α値加算` _targetlenlerp NewParam))
    (set `self.TargetLenLerp` `_加算結果`)
    (else
      (bind `_減算結果` (`self.α値減算` _targetlenlerp NewParam))
      (set `self.TargetLenLerp` `_減算結果`))))

(fn `CameraPosXLerp`
  (params (NewParam :type Boolean))
  (bind _camerapos_x (`KismetMathLibrary.BreakVector` (`self.CameraPos`)))
  (bind _returnvalue_x (`KismetMathLibrary.BreakVector` (`self.K2_GetActorLocation` (`self.GetPlayer`))))
  (if NewParam
    (`self.K2_SetActorLocation` (`KismetMathLibrary.MakeVector` (`KismetMathLibrary.Lerp` _camerapos_x (- _returnvalue_x 500.0) (`self.TargetLenLerp`))))))

(fn `SetLocation`
  (params (Location :type "Vector Structure"))
  (bind _output_get (set `self.CameraPos` (`KismetMathLibrary.MakeVector` (`self.TargetLen`) Location_Y (`self.LocationZ`))))
  (`self.K2_SetActorLocation` _output_get true))

(fn `SetLocation2D`
  (params (Location :type "Vector Structure"))
  (bind _output_get (set `self.LocationZ` (+ Location_Z 120.0)))
  (bind _output_get_2 (set `self.CameraPos` (`KismetMathLibrary.MakeVector` (`self.TargetLen`) Location_Y _output_get)))
  (`self.K2_SetActorLocation` _output_get_2 true))

(fn `SetLocationFirst`
  (params (length :type "Float (double-precision)") (PlayerPos :type "Vector Structure"))
  (bind _output_get (set `self.LocationZ` PlayerPos_Z))
  (bind _output_get_2 (set `self.TargetLen` (- PlayerPos_X length)))
  (bind _output_get_3 (set `self.CameraPos` (`KismetMathLibrary.MakeVector` _output_get_2 PlayerPos_Y _output_get)))
  (`self.K2_SetActorLocation` _output_get_3 true))

(fn `UserConstructionScript`)

(fn `α値加算`
  (params (`加算する変数` :type "Float (double-precision)") (`加算量` :type "Float (double-precision)"))
  (returns (`加算結果` :type "Float (double-precision)"))
  (if (< `加算する変数` 1.0)
    (return (+ `加算する変数` `加算量`))
    (else
      (return `加算する変数`))))

(fn `α値減算`
  (params (`減算する変数` :type "Float (double-precision)") (`減算量` :type "Float (double-precision)"))
  (returns (`減算結果` :type "Float (double-precision)"))
  (if (> `減算する変数` 0.0)
    (return (- `減算する変数` `減算量`))
    (else
      (return `減算する変数`))))