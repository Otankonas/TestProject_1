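; Fixed-depth follow camera that becomes the view target at start, tracking the player's height directly and horizontal Y with lag.
; A short position history supplies the delayed Y while moving, then a stepped lerp catches up once the player stops.
; Timeline events blend its transform toward BossCamera, or its rotation toward BP_NewCamera3, then call that camera's switch event.
; The Camera3 handoff afterwards restores the saved transform and resumes following.
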(event `self.ReceiveBeginPlay`
  (bind _returnvalue (`self.K2_GetActorLocation` (`GameplayStatics.GetPlayerPawn` 0)))
  ;[1 1 1] 初期設定
  (`PlayerController.SetViewTargetWithBlend` (`GameplayStatics.GetPlayerController` 0) self 0.0 "VTBlend_Linear" 0.0 false)
  (`self.SetLocationFirst` 500.0 _returnvalue)
  (set `self.GetPlayerPos` _returnvalue)
  (bind _returnvalue_2 (`GameplayStatics.GetActorOfClass` "/Game/member/Kobayashi/BP/newCamera/BP_NewCamera3.BP_NewCamera3_C"))
  (set `self.AsBP_NewCamera3` _returnvalue_2)
  (set `self.NextPos` (`|MakeArray` _returnvalue (0.0 0.0 0.0) _returnvalue))
  (bind _returnvalue_3 (`GameplayStatics.GetActorOfClass` "/Game/member/Kobayashi/BP/newCamera/BossCamera.BossCamera_C"))
  (set `self.AsBossCamera` _returnvalue_3))

(event `self.ReceiveTick`
  (params (DeltaSeconds :type "Float (single-precision)"))
  (bind (_lerppos_x _lerppos_y) (`KismetMathLibrary.BreakVector` (`self.LerpPos`)))
  (bind (_output_x _output_y) (`KismetMathLibrary.BreakVector` (`|GetArrayItem` (`self.NextPos`) 2)))
  (bind (_returnvalue_x _returnvalue_y _returnvalue_z) (`KismetMathLibrary.BreakVector` (`SceneComponent.K2_GetComponentLocation` (`Character.CapsuleComponent` (`self.As BP Player Base V4`)))))
  (bind (_returnvalue_x_2 _returnvalue_y_2 _returnvalue_z_2) (`KismetMathLibrary.BreakVector` (`SceneComponent.K2_GetComponentLocation` (`Character.CapsuleComponent` (`self.As BP Player Base V4`)))))
  (`self.As BP Player Base V4`
    (:`then`
      _)
    (:`else`
      (bind _asbp_player_base_v4 (cast `/Game/member/Okajima/PlayerSource/BP_PlayerBaseV4` (`GameplayStatics.GetPlayerPawn` 0)))
      (set `self.As BP Player Base V4` _asbp_player_base_v4)))
  (if (== (`|GetArrayItem` (`self.NextPos`)) (`|GetArrayItem` (`self.NextPos`) 1))
    (if (== (`self.LerpTime`) 0.0)
      (set `self.LerpPos` (`|GetArrayItem` (`self.NextPos`) 3)))
    (if (`self.UseCamera4`)
      (`self.K2_SetActorLocation` (`KismetMathLibrary.MakeVector` (`self.LocationDepth`) (`KismetMathLibrary.Lerp` _lerppos_y _returnvalue_y (`self.LerpTime`)) _returnvalue_z)))
    (if (>= (`self.LerpTime`) 0.95)
      (set `self.LerpTime` 0.0)
      (else
        (set `self.LerpTime` (+ (`self.LerpTime`) 0.05))))
    (`KismetArrayLibrary.Array_Insert` (`self.NextPos`) (`KismetMathLibrary.MakeVector` _returnvalue_x_2 _returnvalue_y_2 _returnvalue_z_2))
    (`KismetArrayLibrary.Array_Remove` (`self.NextPos`) 4)
    (set `self.KeepLocation` (`self.K2_GetActorLocation`))
    (set `self.KeepRotation` (`self.K2_GetActorRotation`))
    (else
      (`self.K2_SetActorLocation` (`KismetMathLibrary.MakeVector` (`self.LocationDepth`) _output_y _returnvalue_z))
      (set `self.LerpTime` 0.0)
      (`KismetArrayLibrary.Array_Insert` (`self.NextPos`) (`KismetMathLibrary.MakeVector` _returnvalue_x _returnvalue_y _returnvalue_z))
      (`KismetArrayLibrary.Array_Remove` (`self.NextPos`) 4))))

(event `SetThirdPerson_Event`
  ;[1 1 1] カメラ切り替え
  (`PlayerController.SetViewTargetWithBlend` (`GameplayStatics.GetPlayerController` 0) self 0.0 "VTBlend_Linear" 0.0 false)
  (`KismetSystemLibrary.PrintString` "now4"))

(event `EnterBoss_Event`
  (bind _asbosscamera (`self.AsBossCamera`))
  (bind _keeplocation (`self.KeepLocation`))
  (bind (_keeprotation_roll _keeprotation_pitch _keeprotation_yaw) (`KismetMathLibrary.BreakRotator` (`self.KeepRotation`)))
  (bind (_returnvalue_roll _returnvalue_pitch _returnvalue_yaw) (`KismetMathLibrary.BreakRotator` (`self.K2_GetActorRotation` _asbosscamera)))
  (set `self.UseCamera4` false)
  (bind (_direction _move) (`Timeline|タイムライン_0`)
    (:`Update`
      (`self.K2_SetActorLocationAndRotation` self (+ (* (- (`self.K2_GetActorLocation` _asbosscamera) _keeplocation) _move) _keeplocation) (`KismetMathLibrary.MakeRotator` (+ _keeprotation_roll (* (- _returnvalue_roll _keeprotation_roll) _move)) (+ _keeprotation_pitch (* (- _returnvalue_pitch _keeprotation_pitch) _move)) (+ _keeprotation_yaw (* (- _returnvalue_yaw _keeprotation_yaw) _move))) false false))
    (:`Finished`
      (`KismetSystemLibrary.PrintString` "完了")
      (`/Game/member/Kobayashi/BP/newCamera/BossCamera.SetPointPerson_Event` _asbosscamera))))

(event `ToCamera3_Event`
  (bind (_keeprotation_roll _keeprotation_pitch _keeprotation_yaw) (`KismetMathLibrary.BreakRotator` (`self.KeepRotation`)))
  (bind _asbp_newcamera3 (`self.AsBP_NewCamera3`))
  (bind _keeplocation (`self.KeepLocation`))
  (bind (_returnvalue_roll _returnvalue_pitch _returnvalue_yaw) (`KismetMathLibrary.BreakRotator` (`self.K2_GetActorRotation` _asbp_newcamera3)))
  ;[1 1 1] カメラ切り替え
  (set `self.UseCamera4` false)
  (bind (_direction _move) (`Timeline|タイムライン` :!via `PlayFromStart`)
    (:`Update`
      (`self.K2_SetActorLocationAndRotation` self (+ (* (- (`self.K2_GetActorLocation`) _keeplocation) _move) _keeplocation) (`KismetMathLibrary.MakeRotator` (+ _keeprotation_roll (* (- _returnvalue_roll _keeprotation_roll) _move)) (+ _keeprotation_pitch (* (- _returnvalue_pitch _keeprotation_pitch) _move)) (+ _keeprotation_yaw (* (- _returnvalue_yaw _keeprotation_yaw) _move))) false false))
    (:`Finished`
      (`KismetSystemLibrary.PrintString` "完了")
      (`/Game/member/Kobayashi/BP/newCamera/BP_NewCamera3.SetFirstPerson_Event` _asbp_newcamera3)
      (`self.K2_SetActorLocationAndRotation` (`self.KeepLocation`) (`self.KeepRotation`))
      (set `self.UseCamera4` true))))

(fn `CameraMove`
  (params (A :type "Float (double-precision)"))
  (returns (ReturnValue :type "Float (double-precision)"))
  (bind (_getplayerpos_x _getplayerpos_y) (`KismetMathLibrary.BreakVector` (`self.GetPlayerPos`)))
  (return (+ A (`KismetMathLibrary.Lerp` A _getplayerpos_y 0.1))))

(fn `DistanceFabs`
  (returns (NewParam :type "Float (double-precision)"))
  (bind (_getplayerpos_x _getplayerpos_y) (`KismetMathLibrary.BreakVector` (`self.GetPlayerPos`)))
  (bind (_returnvalue_x _returnvalue_y) (`KismetMathLibrary.BreakVector` (`self.K2_GetActorLocation` self)))
  (bind _returnvalue (- _getplayerpos_y _returnvalue_y))
  (if (< _returnvalue 0.0)
    (return (* _returnvalue -1.0))
    (else
      (return _returnvalue))))

(fn `SetLocationFirst`
  (params (Distance :type "Float (double-precision)") (PlayerPos :type "Vector Structure"))
  (bind _output_get (set `self.LocationVertical` PlayerPos_Z))
  (bind _output_get_2 (set `self.LocationDepth` (- PlayerPos_X Distance)))
  (bind _output_get_3 (set `self.CameraPos` (`KismetMathLibrary.MakeVector` _output_get_2 PlayerPos_Y _output_get)))
  (`self.K2_SetActorLocation` _output_get_3 true))

(fn `UserConstructionScript`)