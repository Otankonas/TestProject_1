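; Test enemy that fights the player through attack, avoid, grabbed and slap-launch reactions, with an HP gauge widget.
; Tick drives a frame-counted state machine with stop-frame delays, reading the player's state to resolve avoids and attack outcomes.
; Idle picks the next action from weighted percentage ranges, and HP thresholds append extra weighted actions.
; A completed grab enters Dead, fades the screen and resets the enemy to its starting spot.
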(event `self.ReceiveBeginPlay`
  (bind _enemystatepattern (`self.EnemyStatePattern`))
  (`|ExecutionSequence`
    (:`then_0`
      (`self.Bind WBP`))
    (:`then_1`
      (set `self.Current State` "NewEnumerator1")
      (set `self.Chance Zone` true)
      (set `self.Anim Frame` 0)
      (set `self.Finish Anim Frame` 0)
      (set `self.Stop Operator Frame` 0))
    (:`then_2`
      (set `self.InitEnmyTransform` (`self.GetTransform`)))
    (:`then_3`
      (if (`KismetArrayLibrary.Array_IsEmpty` _enemystatepattern)
        (`self.SetInitPattern` _enemystatepattern)
        (elif (`KismetArrayLibrary.Array_IsEmpty` (`self.AddActionPattern_A`))
          (set `self.IsEmptyAddFlag` true)
          (else
            (set `self.IsEmptyAddFlag` false))))
      (`self.SetActionPattern` _enemystatepattern))))

(event `Stop Operator`
  (params (`Delay Frame` :type Integer))
  (set `self.Stop Operator Frame` `Delay Frame`))

(event `self.ReceiveAnyDamage`
  (params (Damage :type "Float (single-precision)") (DamageType :type "DamageType Object Reference") (InstigatedBy :type "Controller Object Reference") (DamageCauser :type "Actor Object Reference"))
  (bind _output_get (set `self.HP` (`KismetMathLibrary.FMax` (- (`self.HP`) Damage))))
  (`self.SetAddActionPettern` (`self.IsEmptyAddFlag`) _output_get)
  (if (`KismetMathLibrary.NearlyEqual_FloatFloat` _output_get)
    (`/Game/member/Okajima/wbp/WBP_SampleGageV1.UpdateHealthProgress` (`self.HP Gage`) 0.0)
    (else
      (`/Game/member/Okajima/wbp/WBP_SampleGageV1.UpdateHealthProgress` (`self.HP Gage`) (/ (`self.HP`) (`self.MAXHP`))))))

(event `self.ReceiveTick`
  (params (DeltaSeconds :type "Float (single-precision)"))
  (bind _current_state (`self.Current State`))
  (bind _anim_frame (`self.Anim Frame`))
  (`|ExecutionSequence`
    (:`then_0`
      (`self.execute Stop Operator`)
      (`|ExecutionSequence`
        (:`then_0`
          (`self.Update All State` _anim_frame _current_state)
          (`/Engine/EditorBlueprintResources/StandardMacros.IncrementInt` _anim_frame))
        (:`then_1`
          (`self.is Stop Operator`)
          (if (`|EnumEquality` (`self.Current State`) "NewEnumerator0")
            (`|ExecutionSequence`
              (:`then_0`
                (`KismetSystemLibrary.Delay` (`KismetMathLibrary.RandomFloatInRange` (`self.MinTime`) (`self.MaxTime`)))
                (`self.SetRandomNextAction`)))))
        (:`then_2`
          (`KismetSystemLibrary.PrintString` (`|GetEnumeratorNameAsString` _current_state)))))
    (:`then_1`
      (if (and (`|EnumEquality` (`/Game/member/Okajima/PlayerSource/BP_Player_VerMoment_.Current State` (cast `/Game/member/Okajima/PlayerSource/BP_Player_VerMoment_` (`GameplayStatics.GetPlayerPawn` 0) :!pure true)) "NewEnumerator11") (`|EnumInequality` (`self.Current State`) "NewEnumerator6"))
        (`self.Set Current State` "NewEnumerator2")))))

(event `Attack Event`
  (params (`Current Frame` :type Integer))
  (bind _asbp_player_ver_moment_ (cast `/Game/member/Okajima/PlayerSource/BP_Player_VerMoment_` (`GameplayStatics.GetPlayerPawn` 0) :!pure true))
  (bind _current_state (`/Game/member/Okajima/PlayerSource/BP_Player_VerMoment_.Current State` _asbp_player_ver_moment_))
  (`self.is Animation Now` `Current Frame`
    (:`then`
      (`self.set Anim Default` 30))
    (:`else`
      (if (>= `Current Frame` 15)
        (if (>= `Current Frame` 20)
          (if (`|EnumEquality` _current_state "NewEnumerator13")
            (`self.Set Current State` "NewEnumerator6")
            (elif (or (`|EnumEquality` _current_state "NewEnumerator0") (`|EnumEquality` _current_state "NewEnumerator18"))
              (`self.Set Current State` "NewEnumerator8")
              (`/Game/member/Okajima/PlayerSource/BP_Player_VerMoment_.Set Current State` _asbp_player_ver_moment_ "NewEnumerator19"))))))))

(event `FAILED Event`
  (params (`Current Frame` :type Integer))
  (`self.is Animation Now` `Current Frame`
    (:`then`
      (`self.set Anim Default` 30))))

(event `Avoid Event`
  (params (`Current Frame` :type Integer))
  (`self.is Animation Now` `Current Frame`
    (:`then`
      (`self.set Anim Default` 30))))

(event `Grabbed Event`
  (params (`Current Frame` :type Integer))
  (`self.is Animation Now` `Current Frame`
    (:`then`
      (`self.Set Current State` "NewEnumerator5")
      (`self.isFadeProcess`))
    (:`else`
      (if (>= `Current Frame` 9)
        (set `SkeletalMeshComponent.GlobalAnimRateScale` 0.0 (`self.Mesh`))))))

(event `Dead Event`
  (params (`Current Frame` :type Integer))
  (`self.is Animation Now` `Current Frame`))

(event `Success Event`
  (params (`Current Frame` :type Integer))
  (`self.is Animation Now` `Current Frame`
    (:`then`
      (`self.Set Current State` "NewEnumerator9")
      (`self.Stop Operator` 3))))

(event `Slap Event`
  (params (`Current Frame` :type Integer))
  (bind _capsulecomponent (`Character.CapsuleComponent` (cast `/Game/member/Okajima/PlayerSource/BP_Player_VerMoment_` (`GameplayStatics.GetPlayerPawn` 0) :!pure true)))
  (`self.is Animation Now` (+ `Current Frame` 5)
    (:`then`
      (`PrimitiveComponent.SetCollisionEnabled` _capsulecomponent "QueryAndPhysics")
      (`PrimitiveComponent.AddImpulse` _capsulecomponent (-3000.0 0.0 0.0) "None" true)
      (`self.set Anim Default` 180))
    (:`else`
      (`PrimitiveComponent.SetCollisionEnabled` _capsulecomponent "NoCollision")
      (`SceneComponent.K2_SetWorldLocation` _capsulecomponent (`SceneComponent.GetSocketLocation` (`self.Mesh`) "R_te") true false)
      (`PrimitiveComponent.SetSimulatePhysics` _capsulecomponent true))))

(fn `Bind WBP`
  (bind _aswbp_sample_gage_v1 (cast `/Game/member/Okajima/wbp/WBP_SampleGageV1` (`WidgetComponent.GetUserWidgetObject` (`self.Widget`))))
  (bind _output_get (set `self.HP Gage` _aswbp_sample_gage_v1))
  (`/Game/member/Okajima/wbp/WBP_SampleGageV1.UpdateHealthProgress` _output_get (/ (`self.HP`) (`self.MAXHP`))))

(fn `Set Current State`
  (params (`Next State` :type "/Game/member/Okajima/EnemySource/TestEnemy/BP_TestEnemyAnimState Enum" :default "NewEnumerator0"))
  (set `self.Current State` `Next State`)
  (set `self.Stop Operator Frame` 0)
  (set `self.Anim Frame` 0)
  (switch `/Game/member/Okajima/EnemySource/TestEnemy/BP_TestEnemyAnimState` `Next State`
    (:`NewEnumerator0`
      (set `self.Finish Anim Frame` 0))
    (:`NewEnumerator1`
      (set `self.Finish Anim Frame` 50))
    (:`NewEnumerator2`
      (set `self.Finish Anim Frame` 26))
    (:`NewEnumerator5`
      (set `self.Finish Anim Frame` 0))
    (:`NewEnumerator6`
      (set `self.Finish Anim Frame` 36))
    (:`NewEnumerator7`
      (set `self.Finish Anim Frame` 20))
    (:`NewEnumerator8`
      (set `self.Finish Anim Frame` 48))))

(fn `SetAppendActionPattern`
  (params (AddStatePattern :type "Array of /Game/member/Sugawara/MomentEnemy/BP_EnemyActionAtate Structure"))
  (bind _rangepercent (`self.RangePercent`))
  (if (not (`KismetArrayLibrary.Array_IsEmpty` AddStatePattern))
    (for _index (range (`KismetArrayLibrary.Array_Length` AddStatePattern))
      (bind (_output_enemystate _output_precent) (break `/Game/member/Sugawara/MomentEnemy/BP_EnemyActionAtate` (`|GetArrayItem` AddStatePattern _index)))
      (bind _returnvalue (+ _rangepercent _output_precent))
      (`KismetArrayLibrary.Array_Set` AddStatePattern _index (make `/Game/member/Sugawara/MomentEnemy/BP_EnemyActionAtate` _output_enemystate _output_precent (make `FloatRange` (make `FloatRangeBound` "Exclusive" _rangepercent) (make `FloatRangeBound` "Exclusive" _returnvalue))))
      (set `self.RangePercent` _returnvalue))
    (`KismetArrayLibrary.Array_Append` (`self.EnemyStatePattern`) AddStatePattern)))

(fn `SetInitPattern`
  (params (InitPetten :type "Array of /Game/member/Sugawara/MomentEnemy/BP_EnemyActionAtate Structure"))
  (locals (InitAction :type "/Game/member/Sugawara/MomentEnemy/BP_EnemyActionAtate Structure" :default (struct :`EnemyState` "NewEnumerator1" :`Precent` 10.0 :`RangePercent` (struct :`LowerBound` (struct :`Type` "Exclusive") :`UpperBound` (struct :`Type` "Exclusive")))))
  (`KismetArrayLibrary.Array_Add` InitPetten (`local.InitAction`)))

(fn `Update All State`
  (params (`Current Frame` :type Integer) (`Current State` :type "/Game/member/Okajima/EnemySource/TestEnemy/BP_TestEnemyAnimState Enum" :default "NewEnumerator0"))
  (switch `/Game/member/Okajima/EnemySource/TestEnemy/BP_TestEnemyAnimState` `Current State`
    (:`NewEnumerator1`
      (`self.Attack Event` `Current Frame`))
    (:`NewEnumerator2`
      (`self.Avoid Event` `Current Frame`))
    (:`NewEnumerator5`
      (`self.Dead Event` `Current Frame`))
    (:`NewEnumerator6`
      (`self.FAILED Event` `Current Frame`))
    (:`NewEnumerator7`
      (`self.Grabbed Event` `Current Frame`))
    (:`NewEnumerator8`
      (`self.Success Event` `Current Frame`))
    (:`NewEnumerator9`
      (`self.Slap Event` `Current Frame`))))

(fn `UpdateHPPercent`
  (params (HP :type "Float (double-precision)"))
  (returns (HPPercent :type "Float (double-precision)"))
  (return (* (/ HP (`self.MAXHP`)) 100.0)))

(fn `UserConstructionScript`
  (set `self.HP` (`self.MAXHP`)))