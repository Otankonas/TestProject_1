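; Long-range enemy that sweeps in search of the player, turns to face them and fires charged shots.
; Tick plays a yaw timeline while searching, otherwise smoothly interpolates rotation toward player pawn 0.
; Separate events toggle search, count down charge, spawn BP_Bullet2 at BulletDir and clear cooldown.
; The cooldown check never decrements CoolTimeNow, and the AI stop/restart logic is unconnected.
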(event `self.ReceiveBeginPlay`
  (set `self.IsStop` false)
  (set `self.BaseChageTime` (`self.ChargeTimeNow`))
  (set `self.ActionAttack` false)
  (set `self.Cooltiome` false))

(event `self.ReceiveTick`
  (params (DeltaSeconds :type "Float (single-precision)"))
  ;[1 1 1] プレイヤー回転部分
  (`parent.ReceiveTick` DeltaSeconds)
  (if (`self.ActorRotation`)
    (set `self.PlayerDirectuon` true)
    (bind (_direction _rotation) (`Timeline|タイムライン` :!label _label) ; プレイヤーが見つかるまでの回転部分
      (:`Update`
        (`SceneComponent.K2_SetRelativeRotation` (`self.CapsuleComponent`) (`KismetMathLibrary.MakeRotator` 0.0 0.0 _rotation) false false)))
    (elif (`self.PlayerDirectuon`)
      (set `self.PlayerDirectuon` false)
      (goto _label :!via `Stop`)
      (else
        ;;[1 1 1] プレイヤーを見つけた際の回転部分
        (bind _forward_to_player (`self.CalForward` (`GameplayStatics.GetPlayerPawn` 0)))
        (`SceneComponent.K2_SetWorldRotation` (`self.CapsuleComponent`) _forward_to_player false false)))))

(event `/Game/member/Sugawara/bt/BP_EnemyInterface.Search`
  ;[1 1 1] 回転させる
  (if (not (`self.ActorRotation`))
    (set `self.ActorRotation` true)))

(event `/Game/member/Sugawara/bt/BP_EnemyInterface.StopRotation`
  ;[1 1 1] 回転止める
  (set `self.ActorRotation` false))

(event `/Game/member/Sugawara/bt/BP_EnemyInterface.ChargeTime`
  (bind _returnvalue (- (`self.ChargeTimeNow`) (`self.DeltaTime`)))
  ;[1 1 1] コメント
  (if (`self.Cooltiome`)
    _
    (elif (<= _returnvalue 0.0)
      (set `self.ActionAttack` true)
      (else
        (set `self.ChargeTimeNow` _returnvalue)))))

(event `/Game/member/Sugawara/bt/BP_EnemyInterface.Attack`
  ;[1 1 1] 攻撃関連
  (if (`self.ActionAttack`)
    (`|SpawnActorFromClass` "/Game/member/Sugawara/bt/BP_Bullet2.BP_Bullet2_C" (`SceneComponent.K2_GetComponentToWorld` (`self.BulletDir`)) "AlwaysSpawn" "OverrideRootScale" null null)
    (set `self.Cooltiome` true)
    (set `self.ActionAttack` false)
    (set `self.ChargeTimeNow` (`self.BaseChageTime`))))

(event `/Game/member/Sugawara/bt/BP_EnemyInterface.CoolTime`
  ;[1 1 1] クールタイム時の行動
  (if (`self.Cooltiome`)
    (if (<= (- (`self.CoolTimeNow`) (`self.DeltaTime`)) 0.0)
      (set `self.Cooltiome` false))))

(fn `CalForward`
  (params (Player :type "Pawn Object Reference"))
  (returns (`Forward to Player` :type "Rotator Structure"))
  (return (`KismetMathLibrary.RInterpTo` (`self.K2_GetActorRotation`) (`KismetMathLibrary.FindLookAtRotation` (`self.K2_GetActorLocation`) (`self.K2_GetActorLocation` Player)) (`GameplayStatics.GetWorldDeltaSeconds`) (`self.RotateSpeed`))))

(fn `UserConstructionScript`
  (`parent.UserConstructionScript`))