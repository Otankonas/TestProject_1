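; Close-range sword enemy character whose custom events expose search rotation, charge, attack, cooldown and speed control.
; Tick either plays a yaw timeline to scan or interpolates rotation to face the player.
; Charge countdown arms an attack that, within range, calls the still-empty Blade function, then resets into cooldown after a delay.
; The cooldown check never writes back its timer, and a flag gates walk-speed changes.
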(event `self.ReceiveBeginPlay`
  (set `self.IsStop` false)
  (set `self.BaseChageTime` (`self.ChargeTimeNow`))
  (set `self.ActionAttack` false)
  (set `self.Cooltiome` false))

(event `self.ReceiveTick`
  (params (DeltaSeconds :type "Float (single-precision)"))
  ;[1 1 1] プレイヤー回転部分
  (`|ExecutionSequence`
    (:`then_0`
      (if (`self.ActorRotation`)
        (set `self.PlayerDirectuon` true)
        (bind (_direction _rotation) (`Timeline|タイムライン` :!label _label) ; プレイヤーが見つかるまでの回転部分
          (:`Update`
            (`SceneComponent.K2_SetRelativeRotation` (`self.CapsuleComponent`) (`KismetMathLibrary.MakeRotator` 0.0 0.0 _rotation) false false)))
        (elif (`self.PlayerDirectuon`)
          (set `self.PlayerDirectuon` false)
          (goto _label :!via `Stop`)
          (else
            ;;[1 1 1] プレイヤーを見つけた際の回転部分
            (bind _forward_to_player (`self.CalForward` (`GameplayStatics.GetPlayerPawn` 0)))
            (`SceneComponent.K2_SetWorldRotation` (`self.CapsuleComponent`) _forward_to_player false false)))))))

(event `CustomEvent_1`
  ;[1 1 1] 回転させる
  (if (not (`self.ActorRotation`))
    (set `self.ActorRotation` true)))

(event `CustomEvent_2`
  ;[1 1 1] 回転止める
  (set `self.ActorRotation` false))

(event `CustomEvent_4`
  (bind _returnvalue (- (`self.ChargeTimeNow`) (`self.DeltaTime`)))
  ;[1 1 1] コメント
  (if (`self.Cooltiome`)
    _
    (elif (<= _returnvalue 0.0)
      (set `self.ActionAttack` true)
      (else
        (set `self.ChargeTimeNow` _returnvalue)))))

(event `CustomEvent`
  (bind _attackcollision (`self.AttackCollision`))
  (bind _returnvalue (- (`self.delaytime`) (`self.DeltaTime`)))
  ;[1 1 1] 攻撃関連
  (if (`self.ActionAttack`)
    (`ActorComponent.SetActive` _attackcollision false false)
    (`KismetSystemLibrary.PrintString` "あたり")
    (if (<= (`KismetMathLibrary.VSizeXY` (- (`self.K2_GetActorLocation` self) (`self.K2_GetActorLocation` (`GameplayStatics.GetPlayerPawn` 0)))) (`self.AttackRange`))
      (`self.Blade` self)
      (if (<= _returnvalue 0.0)
        (`KismetSystemLibrary.PrintString` "はジュレ")
        (`ActorComponent.Deactivate` _attackcollision)
        (set `self.Cooltiome` true)
        (set `self.ActionAttack` false)
        (set `self.delaytime` 3.0)
        (set `self.ChargeTimeNow` (`self.BaseChageTime`))
        (else
          (set `self.delaytime` _returnvalue))))))

(event `CustomEvent_3`
  ;[1 1 1] クールタイム時の行動
  (if (`self.Cooltiome`)
    (if (<= (- (`self.CoolTimeNow`) (`self.DeltaTime`)) 0.0)
      (set `self.Cooltiome` false))))

(event `ChangeMoveFlag`
  (params (MoveFlag :type Boolean))
  (set `self.MoveFlag` MoveFlag))

(event `ChangeMove_1`
  (params (ChangeSpeed :type "Float (double-precision)"))
  (if (`self.MoveFlag`)
    (bind _output_get (set `CharacterMovementComponent.MaxWalkSpeed` ChangeSpeed (`self.CharacterMovement`)))
    (set `self.WalkSpeed` _output_get)))

(fn `Blade`)

(fn `CalForward`
  (params (Player :type "Pawn Object Reference"))
  (returns (`Forward to Player` :type "Rotator Structure"))
  (return (`KismetMathLibrary.RInterpTo` (`self.K2_GetActorRotation`) (`KismetMathLibrary.FindLookAtRotation` (`self.K2_GetActorLocation`) (`self.K2_GetActorLocation` Player)) (`GameplayStatics.GetWorldDeltaSeconds`) (`self.RotateSpeed`))))

(fn `UserConstructionScript`)