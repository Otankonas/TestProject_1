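; Close-range enemy character, a child in the old-version grab enemy folder, that turns toward the player and exposes movement and attack events.
; Tick either plays a timeline search spin, toggled by Search and StopRotation, or interpolates rotation to face the player.
; Separate events handle charge and cooldown checks, montage attack, walk speed and strafe mode.
; The range-checked attack sequence and AI logic stop/restart are unconnected, and Blade is empty.
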(event `self.ReceiveBeginPlay`
  (`parent.ReceiveBeginPlay`)
  (set `self.IsStop` false)
  (set `self.BaseChageTime` (`self.ChargeTimeNow`))
  (set `self.ActionAttack` false)
  (set `self.Cooltiome` false))

(event `self.ReceiveTick`
  (params (DeltaSeconds :type "Float (single-precision)"))
  ;[1 1 1] プレイヤー回転部分
  (`parent.ReceiveTick` DeltaSeconds)
  (`|ExecutionSequence`
    (:`then_0`
      (if (`self.ActorRotation`)
        (set `self.PlayerDirectuon` true)
        (bind (_direction _rotation) (`Timeline|タイムライン` :!label _label) ; プレイヤーが見つかるまでの回転部分
          (:`Update`
            (`SceneComponent.K2_SetRelativeRotation` (`self.CapsuleComponent`) (`KismetMathLibrary.MakeRotator` 0.0 0.0 _rotation) false false)))
        (elif (`self.PlayerDirectuon`)
          (set `self.PlayerDirectuon` false)
          (goto _label :!via `Stop`)
          (else
            ;;[1 1 1] プレイヤーを見つけた際の回転部分
            (bind _forward_to_player (`self.CalForward` (`GameplayStatics.GetPlayerPawn` 0)))
            (`SceneComponent.K2_SetWorldRotation` (`self.CapsuleComponent`) _forward_to_player false false)))))))

(event `/Game/member/Sugawara/bt/BP_EnemyInterface.Search`
  ;[1 1 1] 回転させる
  (if (not (`self.ActorRotation`))
    (set `self.ActorRotation` true)))

(event `/Game/member/Sugawara/bt/BP_EnemyInterface.StopRotation`
  ;[1 1 1] 回転止める
  (set `self.ActorRotation` false))

(event `/Game/member/Sugawara/bt/BP_EnemyInterface.ChargeTime`
  (bind _returnvalue (- (`self.ChargeTimeNow`) (`self.DeltaTime`)))
  ;[1 1 1] コメント
  (if (`self.Cooltiome`)
    _
    (elif (<= _returnvalue 0.0)
      (set `self.ActionAttack` true)
      (else
        (set `self.ChargeTimeNow` _returnvalue)))))

(event `/Game/member/Sugawara/bt/BP_EnemyInterface.Attack`
  ;[1 1 1] クールタイム時の行動
  (`|PlayMontage` (`self.Mesh`) "/Game/member/Sugawara/bt/CloseRangeEnemy/AttackMontage.AttackMontage"))

(event `/Game/member/Sugawara/bt/BP_EnemyInterface.CoolTime`
  ;[1 1 1] クールタイム時の行動
  (if (`self.Cooltiome`)
    (if (<= (- (`self.CoolTimeNow`) (`self.DeltaTime`)) 0.0)
      (set `self.Cooltiome` false))))

(event `ChangeMove`
  (params (ChangeSpeed :type "Float (double-precision)"))
  (bind _charactermovement (`self.CharacterMovement`))
  (bind _charactermovement_2 (`self.CharacterMovement`))
  ;[0.2504 0.5366 1] ChangeMove
  (if (`self.CanStrafing`)
    (set `CharacterMovementComponent.bOrientRotationToMovement` false _charactermovement)
    (set `self.bUseControllerRotationYaw` true)
    (else
      (set `CharacterMovementComponent.bOrientRotationToMovement` true _charactermovement)
      (set `self.bUseControllerRotationYaw` false)))
  (if (`self.MoveFlag`)
    (bind _output_get (set `CharacterMovementComponent.MaxWalkSpeed` ChangeSpeed _charactermovement_2))
    (set `self.WalkSpeed` _output_get)
    (else
      (bind _output_get_2 (set `CharacterMovementComponent.MaxWalkSpeed` 0.0 _charactermovement_2))
      (set `self.WalkSpeed` _output_get_2))))

(event `ChangeMoveFlag`
  (params (MoveFlag :type Boolean))
  ;[0.2504 0.5366 1] ChangeMove
  (set `self.MoveFlag` MoveFlag))

(event `/Game/member/Sugawara/bt/BP_EnemyInterface.MoveAction`)

(event `ChangeStrafe`
  (params (CanStrafing :type Boolean))
  (set `self.CanStrafing` CanStrafing))

(fn `Blade`)

(fn `CalForward`
  (params (Player :type "Pawn Object Reference"))
  (returns (`Forward to Player` :type "Rotator Structure"))
  (return (`KismetMathLibrary.RInterpTo` (`self.K2_GetActorRotation`) (`KismetMathLibrary.FindLookAtRotation` (`self.K2_GetActorLocation`) (`self.K2_GetActorLocation` Player)) (`GameplayStatics.GetWorldDeltaSeconds`) (`self.RotateSpeed`))))

(fn `UserConstructionScript`
  (`parent.UserConstructionScript`))