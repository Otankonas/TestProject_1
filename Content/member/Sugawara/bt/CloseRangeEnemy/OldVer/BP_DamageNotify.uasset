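; Animation notify state that opens and closes the sword damage window during a close-range enemy's animations.
; On begin, it casts the mesh owner to BP_CloseRangeGrabBaseV1_Child_2, takes its child actor as BP_SwordCollision and activates that collision.
; On end, it repeats the lookup and deactivates the collision.
; It works only for that specific enemy class, and does nothing if either cast fails.
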(fn `Received_NotifyBegin`
  (params (MeshComp :type "SkeletalMeshComponent Object Reference") (Animation :type "AnimSequenceBase Object Reference") (TotalDuration :type "Float (single-precision)") (EventReference :type "AnimNotifyEventReference Structure (by ref)"))
  (returns (ReturnValue :type Boolean))
  (bind _asbp_close_range_grab_base_v1_child_2 (cast `/Game/member/Sugawara/bt/CloseRangeEnemy/OldVer/BP_CloseRangeGrabBaseV1_Child_2` (`ActorComponent.GetOwner` MeshComp)))
  (bind _assword (cast `/Game/member/Sugawara/bt/CloseRangeEnemy/OldVer/BP_SwordCollision` (`ChildActorComponent.ChildActor` (`/Game/member/Sugawara/bt/CloseRangeEnemy/OldVer/BP_CloseRangeGrabBaseV1_Child_2.ChildActor` _asbp_close_range_grab_base_v1_child_2))))
  (`/Game/member/Sugawara/bt/CloseRangeEnemy/OldVer/BP_SwordCollision.ActiveCollision` _assword)
  (return false))

(fn `Received_NotifyEnd`
  (params (MeshComp :type "SkeletalMeshComponent Object Reference") (Animation :type "AnimSequenceBase Object Reference") (EventReference :type "AnimNotifyEventReference Structure (by ref)"))
  (returns (ReturnValue :type Boolean))
  (bind _asbp_close_range_grab_base_v1_child_2 (cast `/Game/member/Sugawara/bt/CloseRangeEnemy/OldVer/BP_CloseRangeGrabBaseV1_Child_2` (`ActorComponent.GetOwner` MeshComp)))
  (bind _assword (cast `/Game/member/Sugawara/bt/CloseRangeEnemy/OldVer/BP_SwordCollision` (`ChildActorComponent.ChildActor` (`/Game/member/Sugawara/bt/CloseRangeEnemy/OldVer/BP_CloseRangeGrabBaseV1_Child_2.ChildActor` _asbp_close_range_grab_base_v1_child_2))))
  (`/Game/member/Sugawara/bt/CloseRangeEnemy/OldVer/BP_SwordCollision.DeactiveCollision` _assword)
  (return false))