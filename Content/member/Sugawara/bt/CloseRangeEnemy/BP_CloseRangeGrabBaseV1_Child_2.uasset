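; Close-range enemy Blueprint that rotates to search for the player, turns to face them, and runs a charge, attack and cooldown cycle through custom events.
; Tick either plays a yaw timeline while searching or smoothly interpolates rotation toward the player.
; ChargeTime counts down to arm Attack, which checks horizontal range, calls Blade, then enters cooldown after a delay.
; Blade and MoveAction are empty, and CoolTime never decrements its timer.
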(event `self.ReceiveBeginPlay`
  (set `self.IsStop` false)
  (set `self.BaseChageTime` (`self.ChargeTimeNow`))
  (set `self.ActionAttack` false)
  (set `self.Cooltiome` false))

(event `self.ReceiveTick`
  (params (DeltaSeconds :type "Float (single-precision)"))
  ;[1 1 1] プレイヤー回転部分
  (`parent.ReceiveTick` DeltaSeconds)
  (if (`self.ActorRotation`)
    (set `self.PlayerDirectuon` true)
    (bind (_direction _rotation) (`Timeline|タイムライン` :!label _label) ; プレイヤーが見つかるまでの回転部分
      (:`Update`
        (`SceneComponent.K2_SetRelativeRotation` (`self.CapsuleComponent`) (`KismetMathLibrary.MakeRotator` 0.0 0.0 _rotation) false false)))
    (elif (`self.PlayerDirectuon`)
      (set `self.PlayerDirectuon` false)
      (goto _label :!via `Stop`)
      (else
        ;;[1 1 1] プレイヤーを見つけた際の回転部分
        (bind _forward_to_player (`self.CalForward` (`GameplayStatics.GetPlayerPawn` 0)))
        (`SceneComponent.K2_SetWorldRotation` (`self.CapsuleComponent`) _forward_to_player false false)))))

(event `/Game/member/Sugawara/bt/BP_EnemyInterface.Search`
  ;[1 1 1] 回転させる
  (if (not (`self.ActorRotation`))
    (set `self.ActorRotation` true)))

(event `/Game/member/Sugawara/bt/BP_EnemyInterface.StopRotation`
  ;[1 1 1] 回転止める
  (set `self.ActorRotation` false))

(event `/Game/member/Sugawara/bt/BP_EnemyInterface.ChargeTime`
  (bind _returnvalue (- (`self.ChargeTimeNow`) (`self.DeltaTime`)))
  ;[1 1 1] コメント
  (if (`self.Cooltiome`)
    _
    (elif (<= _returnvalue 0.0)
      (set `self.ActionAttack` true)
      (else
        (set `self.ChargeTimeNow` _returnvalue)))))

(event `/Game/member/Sugawara/bt/BP_EnemyInterface.Attack`
  (bind _attackcollision (`self.AttackCollision`))
  (bind _returnvalue (- (`self.delaytime`) (`self.DeltaTime`)))
  ;[1 1 1] 攻撃関連
  (if (`self.ActionAttack`)
    (`ActorComponent.SetActive` _attackcollision false false)
    (`KismetSystemLibrary.PrintString` "あたり")
    (if (<= (`KismetMathLibrary.VSizeXY` (- (`self.K2_GetActorLocation` self) (`self.K2_GetActorLocation` (`GameplayStatics.GetPlayerPawn` 0)))) (`self.AttackRange`))
      (`self.Blade` self)
      (if (<= _returnvalue 0.0)
        (`KismetSystemLibrary.PrintString` "はジュレ")
        (`ActorComponent.Deactivate` _attackcollision)
        (set `self.Cooltiome` true)
        (set `self.ActionAttack` false)
        (set `self.delaytime` 3.0)
        (set `self.ChargeTimeNow` (`self.BaseChageTime`))
        (else
          (set `self.delaytime` _returnvalue))))))

(event `/Game/member/Sugawara/bt/BP_EnemyInterface.CoolTime`
  ;[1 1 1] クールタイム時の行動
  (if (`self.Cooltiome`)
    (if (<= (- (`self.CoolTimeNow`) (`self.DeltaTime`)) 0.0)
      (set `self.Cooltiome` false))))

(event `self.AttackCollision.OnComponentHit`
  (params (HitComponent :type "PrimitiveComponent Object Reference") (OtherActor :type "Actor Object Reference") (OtherComp :type "PrimitiveComponent Object Reference") (NormalImpulse :type "Vector Structure") (Hit :type "HitResult Structure (by ref)"))
  (`KismetSystemLibrary.PrintString` (`KismetSystemLibrary.GetDisplayName` OtherActor)))

(event `/Game/member/Sugawara/bt/BP_EnemyInterface.MoveAction`)

(fn `Blade`)

(fn `CalForward`
  (params (Player :type "Pawn Object Reference"))
  (returns (`Forward to Player` :type "Rotator Structure"))
  (return (`KismetMathLibrary.RInterpTo` (`self.K2_GetActorRotation`) (`KismetMathLibrary.FindLookAtRotation` (`self.K2_GetActorLocation`) (`self.K2_GetActorLocation` Player)) (`GameplayStatics.GetWorldDeltaSeconds`) (`self.RotateSpeed`))))

(fn `UserConstructionScript`
  (`parent.UserConstructionScript`))