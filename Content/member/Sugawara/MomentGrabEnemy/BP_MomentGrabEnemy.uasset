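; BP_MomentGrabEnemy is an enemy for a quick-draw reaction duel against the player.
; Tick counts down to an exclamation-mark cue, attacks if the player jumps early, otherwise opens a random-length Delay window.
; A player attack after that delay marks the enemy for destruction; none makes it attack, with EnemyState tracking each phase.
; Tick also clears PlayerAttackFlag where player attack input is meant to arrive; nothing here sets it true.
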(event `self.ReceiveBeginPlay`
  (bind _ascharacter (cast `Character` (`GameplayStatics.GetPlayerPawn` 0)))
  (set `self.As Character` _ascharacter)
  (set `self.AttackFlag` false)
  (set `self.DeleteFlag` false)
  (set `self.SetTime` (`KismetMathLibrary.RandomFloatInRange` (`self.MinTime`) (`self.MaxTime`)))
  (set `self.EnemyState` "NewEnumerator0")
  (set `self.WaitTime` 10.0))

(event `self.ReceiveTick`
  (params (DeltaSeconds :type "Float (single-precision)"))
  (bind _returnvalue (- (`self.WaitTime`) (`self.DelayTime`)))
  (`|ExecutionSequence`
    (:`then_0`
      ;[1 1 1] ビックリマークまでの時間まで待つ
      (set `self.EnemyState` "NewEnumerator4")
      (if (< _returnvalue 0.0)
        ;[1 1 1] お手つきした場合
        (if (`self.PlayerAttackFlag`)
          ;[1 1 1] 攻撃判定をする
          (set `self.EnemyState` "NewEnumerator1")
          (set `self.AttackFlag` true)
          (else
            ;[1 1 1] プレイヤーの攻撃時間待ち
            (set `self.EnemyState` "NewEnumerator5")
            (`KismetSystemLibrary.Delay` (`self.SetTime`))
            (if (`self.PlayerAttackFlag`)
              ;[1 1 1] 負けた場合のやられるフラグを立てる
              (set `self.EnemyState` "NewEnumerator3")
              (set `self.DeleteFlag` true)
              (else
                ;[1 1 1] 勝った時の攻撃フラグを立てる
                (set `self.EnemyState` "NewEnumerator0")
                (set `self.AttackFlag` true)))))
        (else
          (set `self.WaitTime` _returnvalue))))
    (:`then_1`
      ;[1 1 1] プレイヤーから攻撃情報を受け取る
      (set `self.PlayerAttackFlag` false))
    (:`then_2`
      ;[1 1 1] やられるフラグ
      (if (`self.DeleteFlag`)
        (`self.K2_DestroyActor`)))))

(fn `UserConstructionScript`)