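; Close-range enemy character driven by a frame-counted state machine covering idle, search, find, attack, guard, damage, grab, avoid and death.
; Tick dispatches the current state's event; SetCurrentState resets the frame counter and sets each state's length, after which timed actions generally return to Idle.
; States rotate to scan or face the player, while grab uses animation-stop macros and applies accumulated damage to HP.
; Player-state reactions and MoveEvent dispatch are unwired.
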(event `self.ReceiveBeginPlay`
  ;[1 1 1] 初期化
  (`parent.ReceiveBeginPlay`)
  (`|ExecutionSequence`
    (:`then_0`
      (set `self.NowAnimationFlame` 0)
      (set `self.FinishAnimFlame` 0)
      (set `self.CurrentEnemyState` "NewEnumerator0")
      (set `self.CurrentStopAnimationFlag` false)
      (bind _output_get (set `self.MaxHP` 100))
      (set `self.HP` _output_get)
      (set `self.MultiBoxCheckDistance` 10.0)
      (set `self.LineCheckDistance` (30.0 50.0)))
    (:`then_1`
      (bind _asbp_player_base_v4 (cast `/Game/member/Okajima/PlayerSource/BP_PlayerBaseV4` (`GameplayStatics.GetPlayerPawn` 0)))
      (set `self.PlayerCurrent State` (`/Game/member/Okajima/PlayerSource/BP_PlayerBaseV4.Current State` _asbp_player_base_v4))
      ;[1 1 1] プレイヤーのダメージ値
      (set `self.PlayerAttack` 10))))

(event `self.ReceiveTick`
  (params (DeltaSeconds :type "Float (single-precision)"))
  (bind _nowanimationflame (`self.NowAnimationFlame`))
  (`parent.ReceiveTick` DeltaSeconds)
  (`|ExecutionSequence`
    (:`then_0`
      (`self.UpdateAllState` (`self.CurrentEnemyState`) _nowanimationflame)
      (`KismetSystemLibrary.PrintString` "Hello")
      (`/Engine/EditorBlueprintResources/StandardMacros.IncrementInt` _nowanimationflame))))

(event `IdleEvent`
  (params (CuurrentFlame :type Integer))
  (`self.CallForward`))

(event `GrabedEvent`
  (params (DeadEvent :type Integer))
  (bind _mesh (`self.Mesh`))
  (`self.IsStopAnimation` 30
    (:`then`
      (`|ExecutionSequence`
        (:`then_0`
          (`self.Is Animation Now` DeadEvent
            (:` `
              (set `SkeletalMeshComponent.GlobalAnimRateScale` 1.0 _mesh)
              (`self.Set Current State` "NewEnumerator0")
              (goto _label :!via `Reset`))
            (:`false`
              (set `SkeletalMeshComponent.GlobalAnimRateScale` 0.0 _mesh))))
        (:`then_1`
          (`/Engine/EditorBlueprintResources/StandardMacros.DoOnce` false :!label _label
            (:`Completed`
              (set `self.HP` (- (`self.HP`) (`self.Accumulated damage`))))))
        (:`then_2`
          (if (<= (`self.HP`) 0)
            (`self.Set Current State` "NewEnumerator10")
            (goto _label :!via `Reset`)))))))

(event `DeadEvent`
  (params (CuurrentFlame :type Integer))
  (set `SkeletalMeshComponent.GlobalAnimRateScale` 0.0 (`self.Mesh`)))

(event `DamageEvent`
  (params (CuurrentFlame :type Integer))
  (`self.Is Animation Now` CuurrentFlame
    (:` `
      (`|ExecutionSequence`
        (:`then_0`
          (`self.Set Current State` "NewEnumerator0"))
        (:`then_1`
          (goto _label_2 :!via `Reset`))))
    (:`false`
      (`/Engine/EditorBlueprintResources/StandardMacros.DoOnce` false :!label _label_2
        (:`Completed`
          (set `self.Accumulated damage` (+ (`self.PlayerAttack`) (`self.Accumulated damage`))))))))

(event `AvoidEvent`
  (params (CuurrentFlame :type Integer))
  (`self.Is Animation Now` CuurrentFlame
    (:` `
      (`self.Set Current State` "NewEnumerator0"))))

(event `Search`
  (`self.Excute Rotation Component` :!label _label_3))

(event `Find`
  (`|ExecutionSequence`
    (:`then_0`
      (goto _label_3 :!via `stop`))
    (:`then_1`
      (`self.CallForward`))))

(event `AttackEvent`
  (params (Nowflame :type Integer))
  (`self.Is Animation Now` Nowflame
    (:` `
      (`self.Set Current State` "NewEnumerator0"))
    (:`false`
      (if (> Nowflame 8)
        _))))

(event `MoveEvent`
  (params (Nowflame :type Integer))
  (`self.CallForward`)
  (`self.Is Animation Now` Nowflame
    (:` `
      (`self.Set Current State` "NewEnumerator0"))))

(event `GurdeEvent`
  (params (Nowflame :type Integer))
  (`self.CallForward`)
  (`self.Is Animation Now` Nowflame
    (:` `
      (`self.Set Current State` "NewEnumerator0"))))

(event `JudgeEvent`
  (bind _asbp_player_base_v4 (cast `/Game/member/Okajima/PlayerSource/BP_PlayerBaseV4` (`GameplayStatics.GetPlayerPawn` 0) :!pure true))
  (if (`|EnumEquality` (`self.CurrentEnemyState`) "NewEnumerator4")
    (`/Game/member/Okajima/PlayerSource/BP_PlayerBaseV4.Set Current State` _asbp_player_base_v4 "NewEnumerator0")
    (set `/Game/member/Okajima/PlayerSource/BP_PlayerBaseV4.LockOn` true _asbp_player_base_v4)
    (else
      (`self.Set Current State` "NewEnumerator0"))))

(event `SetMoveEvent`
  (params (MoveDirection :type "/Game/member/Sugawara/Enemy/CloseRangeEnemy/MoveDirection Enum" :default "NewEnumerator0"))
  (set `self.MoveDirection` MoveDirection)
  (set `self.MoveSpeed` (`KismetMathLibrary.RandomFloatInRange` (`self.MinMoveSpeed`) (`self.MaxMoveSpeed`)))
  (set `self.FinishAnimFlame` (`KismetMathLibrary.RandomIntegerInRange` (`self.MinMoveFlame`) (`self.MaxMoveFlame`))))

(fn `CallForward`
  (`self.K2_SetActorRotation` (`KismetMathLibrary.RInterpTo` (`self.K2_GetActorRotation`) (`KismetMathLibrary.FindLookAtRotation` (`self.K2_GetActorLocation`) (`self.K2_GetActorLocation` (`GameplayStatics.GetPlayerPawn` 0))) (`GameplayStatics.GetWorldDeltaSeconds`) (`self.RotateSpeed`)))
  (return))

(fn `Set Current State`
  (params (SetState :type "/Game/member/Sugawara/Enemy/CloseRangeEnemy/CloseEnemyState Enum" :default "NewEnumerator0"))
  (set `self.IsStopFlag` false)
  (bind _output_get (set `self.CurrentEnemyState` SetState))
  (set `self.NowAnimationFlame` 0)
  (switch `/Game/member/Sugawara/Enemy/CloseRangeEnemy/CloseEnemyState` _output_get
    (:`NewEnumerator0`
      (set `self.FinishAnimFlame` 0))
    (:`NewEnumerator1`
      (set `self.FinishAnimFlame` 0))
    (:`NewEnumerator13`
      (set `self.FinishAnimFlame` 0))
    (:`NewEnumerator3`
      (set `self.FinishAnimFlame` 50))
    (:`NewEnumerator4`
      (set `self.FinishAnimFlame` 20))
    (:`NewEnumerator11`
      (set `self.FinishAnimFlame` 18))
    (:`NewEnumerator9`
      (set `self.FinishAnimFlame` 0))
    (:`NewEnumerator10`
      (set `self.FinishAnimFlame` 17))
    (:`NewEnumerator12`
      (set `self.FinishAnimFlame` 3))))

(fn `SetRandom`
  (returns (SetNumber :type Integer))
  (return (`KismetMathLibrary.RandomIntegerInRange` 0 (`self.MaxRandomFloat`))))

(fn `UpdateAllState`
  (params (NowState :type "/Game/member/Sugawara/Enemy/CloseRangeEnemy/CloseEnemyState Enum" :default "NewEnumerator0") (NowFlame :type Integer))
  (switch `/Game/member/Sugawara/Enemy/CloseRangeEnemy/CloseEnemyState` NowState
    (:`NewEnumerator0`
      (`self.IdleEvent` NowFlame))
    (:`NewEnumerator1`
      (`self.Search`))
    (:`NewEnumerator13`
      (`self.Find`))
    (:`NewEnumerator3`
      (`self.AttackEvent` NowFlame))
    (:`NewEnumerator4`
      (`self.GurdeEvent` NowFlame))
    (:`NewEnumerator11`
      (`self.DamageEvent` NowFlame))
    (:`NewEnumerator9`
      (`self.GrabedEvent` NowFlame))
    (:`NewEnumerator10`
      (`self.DeadEvent` NowFlame))
    (:`NewEnumerator12`
      (`self.AvoidEvent` NowFlame))))

(fn `UserConstructionScript`
  (`parent.UserConstructionScript`))