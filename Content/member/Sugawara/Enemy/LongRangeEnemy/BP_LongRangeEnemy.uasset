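; Long-range enemy actor that reacts to the player's grabs and hits; no ranged attack logic is present.
; Tick runs a frame-counted state machine (Idle, Search, Damage, Grabed, Dead, Avoid) and polls the player's state enum to trigger Damage or Grabed.
; Hits only add to AccumulatedDamage, which is subtracted from HP when a grab ends, leading to Dead at zero.
; Grabs use a frame-count stop and freeze the mesh animation rate.
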(event `self.ReceiveBeginPlay`
  ;[1 1 1] 初期化
  (`parent.ReceiveBeginPlay`)
  (`|ExecutionSequence`
    (:`then_0`
      (set `self.NowAnimationFlame` 0)
      (set `self.FinishAnimFlame` 0)
      (set `self.CurrentEnemyState` "NewEnumerator0")
      (set `self.CurrentStopAnimationFlag` false)
      (bind _output_get (set `self.MaxHP` 100))
      (set `self.HP` _output_get))
    (:`then_1`
      (bind _asbp_player_base_v4 (cast `/Game/member/Okajima/PlayerSource/BP_PlayerBaseV4` (`GameplayStatics.GetPlayerPawn` 0)))
      (set `self.PlayerCurrent State` (`/Game/member/Okajima/PlayerSource/BP_PlayerBaseV4.Current State` _asbp_player_base_v4))
      ;[1 1 1] プレイヤーのダメージ値
      (set `self.PlayerAttack` 10))))

(event `self.ReceiveTick`
  (params (DeltaSeconds :type "Float (single-precision)"))
  (bind _currentenemystate (`self.CurrentEnemyState`))
  (bind _nowanimationflame (`self.NowAnimationFlame`))
  (`parent.ReceiveTick` DeltaSeconds)
  (`|ExecutionSequence`
    (:`then_0`
      (`self.UpdateAllState` _currentenemystate _nowanimationflame)
      (`KismetSystemLibrary.PrintString` (`|GetEnumeratorNameAsString` _currentenemystate))
      (`/Engine/EditorBlueprintResources/StandardMacros.IncrementInt` _nowanimationflame))
    (:`then_2`
      ;[1 1 1] ステータス確認用（プレイヤーのステータス参照）
      (`|ExecutionSequence`
        (:`then_0`
          (set `self.PlayerCurrent State` (`/Game/member/Okajima/PlayerSource/BP_PlayerBaseV4.Current State` (cast `/Game/member/Okajima/PlayerSource/BP_PlayerBaseV4` (`GameplayStatics.GetPlayerPawn` 0) :!pure true))))
        (:`then_1`
          (if (`|EnumEquality` (`self.PlayerCurrent State`) "NewEnumerator8")
            (`/Engine/EditorBlueprintResources/StandardMacros.DoOnce` false :!label _label
              (:`Completed`
                (`self.Set Current State` "NewEnumerator9")))
            (else
              (goto _label :!via `Reset`))))
        (:`then_2`
          (if (`|EnumEquality` (`self.PlayerCurrent State`) "NewEnumerator4")
            (`/Engine/EditorBlueprintResources/StandardMacros.DoOnce` false :!label _label_2
              (:`Completed`
                (`self.Set Current State` "NewEnumerator11" :!label _label_3)))
            (else
              (goto _label_2 :!via `Reset`))))
        (:`then_3`
          (if (`|EnumEquality` (`self.PlayerCurrent State`) "NewEnumerator5")
            (`/Engine/EditorBlueprintResources/StandardMacros.DoOnce` false :!label _label_4
              (:`Completed`
                (goto _label_3)))
            (else
              (goto _label_4 :!via `Reset`))))
        (:`then_4`
          (if (`|EnumEquality` (`self.PlayerCurrent State`) "NewEnumerator6")
            (`/Engine/EditorBlueprintResources/StandardMacros.DoOnce` false :!label _label_5
              (:`Completed`
                (goto _label_3)))
            (else
              (goto _label_5 :!via `Reset`))))))))

(event `IdleEvent`
  (params (CuurrentFlame :type Integer)))

(event `GrabedEvent`
  (params (DeadEvent :type Integer))
  (bind _mesh (`self.Mesh`))
  (`self.IsStopAnimation` 30
    (:`then`
      (`|ExecutionSequence`
        (:`then_0`
          (`self.Is Animation Now` DeadEvent
            (:` `
              (set `SkeletalMeshComponent.GlobalAnimRateScale` 1.0 _mesh)
              (`self.Set Current State` "NewEnumerator0")
              (goto _label :!via `Reset`))
            (:`false`
              (set `SkeletalMeshComponent.GlobalAnimRateScale` 0.0 _mesh))))
        (:`then_1`
          (`/Engine/EditorBlueprintResources/StandardMacros.DoOnce` false :!label _label
            (:`Completed`
              (set `self.HP` (- (`self.HP`) (`self.Accumulated damage`))))))
        (:`then_2`
          (if (<= (`self.HP`) 0)
            (`self.Set Current State` "NewEnumerator10")
            (goto _label :!via `Reset`)))))))

(event `DeadEvent`
  (params (CuurrentFlame :type Integer))
  (set `SkeletalMeshComponent.GlobalAnimRateScale` 0.0 (`self.Mesh`)))

(event `DamageEvent`
  (params (CuurrentFlame :type Integer))
  (`self.Is Animation Now` CuurrentFlame
    (:` `
      (`|ExecutionSequence`
        (:`then_0`
          (`self.Set Current State` "NewEnumerator0"))
        (:`then_1`
          (goto _label_2 :!via `Reset`))))
    (:`false`
      (`/Engine/EditorBlueprintResources/StandardMacros.DoOnce` false :!label _label_2
        (:`Completed`
          (set `self.Accumulated damage` (+ (`self.PlayerAttack`) (`self.Accumulated damage`))))))))

(event `AvoidEvent`
  (params (CuurrentFlame :type Integer))
  (`self.Is Animation Now` CuurrentFlame
    (:` `
      (`self.Set Current State` "NewEnumerator0"))))

(event `Search`
  (bind (_direction _directiontime) (`Timeline|PlayerRotation`)
    (:`Update`
      (`self.K2_SetActorRotation` (`KismetMathLibrary.MakeRotator` 0.0 0.0 _directiontime)))))

(fn `Set Current State`
  (params (SetState :type "/Game/member/Sugawara/Enemy/EnemyState Enum" :default "NewEnumerator0"))
  (set `self.IsStopFlag` false)
  (bind _output_get (set `self.CurrentEnemyState` SetState))
  (set `self.NowAnimationFlame` 0)
  (switch `/Game/member/Sugawara/Enemy/EnemyState` _output_get
    (:`NewEnumerator0`
      (set `self.FinishAnimFlame` 0))
    (:`NewEnumerator11`
      (set `self.FinishAnimFlame` 3))
    (:`NewEnumerator9`
      (set `self.FinishAnimFlame` 18))
    (:`NewEnumerator10`
      (set `self.FinishAnimFlame` 0))
    (:`NewEnumerator12`
      (set `self.FinishAnimFlame` 17))))

(fn `UpdateAllState`
  (params (NowState :type "/Game/member/Sugawara/Enemy/EnemyState Enum" :default "NewEnumerator0") (NowFlame :type Integer))
  (switch `/Game/member/Sugawara/Enemy/EnemyState` NowState
    (:`NewEnumerator0`
      (`self.IdleEvent` NowFlame))
    (:`NewEnumerator1`
      (`self.Search`))
    (:`NewEnumerator11`
      (`self.DamageEvent` NowFlame))
    (:`NewEnumerator9`
      (`self.GrabedEvent` NowFlame))
    (:`NewEnumerator10`
      (`self.DeadEvent` NowFlame))
    (:`NewEnumerator12`
      (`self.AvoidEvent` NowFlame))))

(fn `UserConstructionScript`
  (`parent.UserConstructionScript`))