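; BP_StageSlectData is an actor that holds a StageData array and serves as a lookup for stage data by stage number.
; GetSelectStageData treats the number as 1-based, checks it against the array bounds, and returns the matching entry with a success flag.
; Out-of-range numbers report failure, and the event graph and construction script contain no logic.
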(fn `Get Select Stage Data`
  (params (`Stage Num` :type Integer))
  (returns (Return :type "/Game/member/Oshiro/sangaku/stageselectTest/StageSelectData Structure") (`Return Success` :type Boolean))
  (bind _stage_data (`self.Stage Data`))
  (if (> `Stage Num` 0)
    (if (<= `Stage Num` (`KismetArrayLibrary.Array_Length` _stage_data))
      (set `self.Return Stage Data` (`|GetArrayItem` _stage_data (- `Stage Num` 1)))
      (set `self.Success` true)
      (else
        (set `self.Success` false :!label _label)))
    (else
      (goto _label)))
  (return (`self.Return Stage Data`) (`self.Success`)))

(fn `UserConstructionScript`)