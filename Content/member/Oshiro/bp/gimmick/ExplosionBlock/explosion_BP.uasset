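; Explosive block gimmick that explodes the first time something hits its Geometry Collection component.
; The hit enables physics on the touching component unless it belongs to the player pawn, then spawns a temporary FS_MasterField with configurable radius and magnitude, triggering it before destroying it.
; Explosion and steam particles play at the block, and a flag blocks repeat triggers.
; Tick destroys the block after a configurable delay.
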(event `self.ReceiveBeginPlay`
  ;[1 1 1] 初期化
  (set `self.Expflag` false))

(event `self.explosionblock_GC.OnComponentHit`
  (params (HitComponent :type "PrimitiveComponent Object Reference") (OtherActor :type "Actor Object Reference") (OtherComp :type "PrimitiveComponent Object Reference") (NormalImpulse :type "Vector Structure") (Hit :type "HitResult Structure (by ref)"))
  (bind _returnvalue (`self.K2_GetActorLocation`))
  (bind _effectscale (`self.EffectScale`))
  ;[1 1 1] 爆発処理(何かが触れたら爆発)
  (if (not (`self.Expflag`))
    (if (not (== OtherActor (`GameplayStatics.GetPlayerPawn` 0)))
      (`PrimitiveComponent.SetSimulatePhysics` OtherComp true))
    (bind _returnvalue_2 (`|SpawnActorFromClass` "/Engine/EditorResources/FieldNodes/FS_MasterField.FS_MasterField_C" (`KismetMathLibrary.MakeTransform` (`self.K2_GetActorLocation`)) "Undefined" "OverrideRootScale" null null))
    (`SphereComponent.SetSphereRadius` (`/Engine/EditorResources/FieldNodes/FS_MasterField.SphereVolumeCol` _returnvalue_2) (`self.Explosion Radius`) true)
    (set `/Engine/EditorResources/FieldNodes/FS_MasterField.Radial Magnitude` (`self.Explosion Power`) _returnvalue_2)
    (`/Engine/EditorResources/FieldNodes/FS_MasterField.CE_Trigger` _returnvalue_2)
    (`self.K2_DestroyActor` _returnvalue_2)
    (set `self.Expflag` true)
    ;[1 1 1] エフェクト部分
    (`GameplayStatics.SpawnEmitterAtLocation` "/Game/StarterContent/Particles/P_Explosion.P_Explosion" _returnvalue (struct) _effectscale)
    (`GameplayStatics.SpawnEmitterAtLocation` "/Game/StarterContent/Particles/P_Steam_Lit.P_Steam_Lit" _returnvalue (struct) _effectscale)))

(event `self.ReceiveTick`
  (params (DeltaSeconds :type "Float (single-precision)"))
  ;[1 1 1] オブジェクト破棄処理
  (if (`self.Expflag`)
    (`KismetSystemLibrary.Delay` (`self.Destorytime`))
    (`self.K2_DestroyActor`)))

(fn `UserConstructionScript`)