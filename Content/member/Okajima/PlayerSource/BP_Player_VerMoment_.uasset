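; Player character Blueprint for a grab-and-slap combat prototype, with dodge, health gauge, and a fade-out reset after being grabbed.
; Tick drives a frame-counted state machine: each state sets a length, dispatches its event, and uses recovery-frame countdowns to gate input.
; Grab attacks check the first test enemy's state to fail or succeed; success leads to a slap that carries the enemy on a hand socket, then launches it.
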(event `self.ReceiveBeginPlay`
  ;[0 0.001895 1] Initialize
  (`|ExecutionSequence`
    (:`then_0`
      (`self.Bind Input Actions`))
    (:`then_1`
      (`self.Bind WBP`))
    (:`then_2`
      (set `self.Current State` "NewEnumerator0")
      (set `self.Chance Zone` true)
      (set `self.Anim Frame` 0)
      (set `self.Finish Anim Frame` 0)
      (set `self.Stop Operator Frame` 0))
    (:`then_3`
      (bind _outactors (`GameplayStatics.GetAllActorsOfClass` "/Game/member/Sugawara/MomentEnemy/BP_TestEnemy_VerMoment_CopyVer.BP_TestEnemy_VerMoment_CopyVer_C"))
      (set `self.Out Actors` _outactors))
    (:`then_4`
      (set `self.InitPlayerTransform` (`self.GetTransform`)))))

(event `Stop Operator`
  (params (`Delay Frame` :type Integer))
  ;[0 0.5834 1] Set Rigidity
  (set `self.Stop Operator Frame` `Delay Frame`))

(event `self.ReceiveAnyDamage`
  (params (Damage :type "Float (single-precision)") (DamageType :type "DamageType Object Reference") (InstigatedBy :type "Controller Object Reference") (DamageCauser :type "Actor Object Reference"))
  ;[0 1 0.3704] Set Damage
  (bind _output_get (set `self.HP` (`KismetMathLibrary.FMax` (- (`self.HP`) Damage))))
  (if (`KismetMathLibrary.NearlyEqual_FloatFloat` _output_get)
    (`/Game/member/Okajima/wbp/WBP_SampleGageV1.UpdateHealthProgress` (`self.HP Gage`) 0.0)
    (else
      (`/Game/member/Okajima/wbp/WBP_SampleGageV1.UpdateHealthProgress` (`self.HP Gage`) (/ (`self.HP`) (`self.MAXHP`))))))

(event `self.ReceiveTick`
  (params (DeltaSeconds :type "Float (single-precision)"))
  (bind _anim_frame (`self.Anim Frame`))
  (`self.execute Stop Operator`)
  (`|ExecutionSequence`
    (:`then_0`
      (`self.Update All State` _anim_frame (`self.Current State`))
      (`/Engine/EditorBlueprintResources/StandardMacros.IncrementInt` _anim_frame))))

(event `Key|Zero`
  (params (Key :type "Key Structure"))
  (:`Pressed`
    (`/Game/member/Sugawara/MomentEnemy/BP_TestEnemy_VerMoment_CopyVer.Set Current State` (`|GetArrayItem` (`self.Out Actors`)) "NewEnumerator2")))

(event `EnhancedInput|/Game/DefaultSetting/inputAction/IA_Attack`
  (params (ActionValue :type Boolean) (ElapsedSeconds :type "Float (double-precision)") (TriggeredSeconds :type "Float (double-precision)") (InputAction :type "InputAction Object Reference" :default "/Game/DefaultSetting/inputAction/IA_Attack.IA_Attack"))
  (:`Started`
    (`self.is Stop Operator`)
    (`self.is Not Grab`
      (:`else`
        (if (`|EnumInequality` (`self.Current State`) "NewEnumerator17")
          (`self.Set Current State` "NewEnumerator11"))))))

(event `EnhancedInput|/Game/DefaultSetting/inputAction/IA_Avoidance`
  (params (ActionValue :type Boolean) (ElapsedSeconds :type "Float (double-precision)") (TriggeredSeconds :type "Float (double-precision)") (InputAction :type "InputAction Object Reference" :default "/Game/DefaultSetting/inputAction/IA_Avoidance.IA_Avoidance"))
  (bind _current_state (`self.Current State`))
  (:`Started`
    (`self.is Stop Operator`)
    (if (and (`|EnumInequality` _current_state "NewEnumerator14") (`|EnumInequality` _current_state "NewEnumerator12") (`|EnumInequality` _current_state "NewEnumerator17"))
      (`self.is Not Avoidance`
        (:`else`
          (`self.Set Current State` "NewEnumerator13"))))))

(event `Moment Attack Event`
  (params (`Current Frame` :type Integer))
  (bind _current_state (`/Game/member/Sugawara/MomentEnemy/BP_TestEnemy_VerMoment_CopyVer.Current State` (`|GetArrayItem` (`self.Out Actors`))))
  (`self.is Animation Now` `Current Frame`
    (:`then`
      (`self.set Anim Default` 30))
    (:`else`
      (set `SkeletalMeshComponent.GlobalAnimRateScale` 2.0 (`self.Mesh`))
      (if (>= `Current Frame` 3)
        (if (>= `Current Frame` 7)
          (if (`|EnumEquality` _current_state "NewEnumerator2")
            (`self.Set Current State` "NewEnumerator18")
            (else
              (set `SkeletalMeshComponent.GlobalAnimRateScale` 1.0 (`self.Mesh`))
              (if (`|EnumEquality` _current_state "NewEnumerator6")
                (`self.Set Current State` "NewEnumerator12")
                (`/Game/member/Sugawara/MomentEnemy/BP_TestEnemy_VerMoment_CopyVer.Set Current State` (`|GetArrayItem` (`self.Out Actors`)) "NewEnumerator7")))))))))

(event `Grabbed Event`
  (params (`Current Frame` :type Integer))
  (`self.is Animation Now` `Current Frame`
    (:`then`
      (`self.Set Current State` "NewEnumerator17")
      (`self.IsFadeProcess`))
    (:`else`
      (if (>= `Current Frame` 9)
        (set `SkeletalMeshComponent.GlobalAnimRateScale` 0.0 (`self.Mesh`))))))

(event `FAILED Event`
  (params (`Current Frame` :type Integer))
  (`self.is Animation Now` `Current Frame`
    (:`then`
      (set `SkeletalMeshComponent.GlobalAnimRateScale` 1.0 (`self.Mesh`))
      (`self.set Anim Default` 30))
    (:`else`
      (set `SkeletalMeshComponent.GlobalAnimRateScale` 3.0 (`self.Mesh`)))))

(event `Avoidance Event`
  (params (`Current Frame` :type Integer))
  (`self.is Animation Now` `Current Frame`
    (:`then`
      (`self.set Anim Default` 5))))

(event `Success Event`
  (params (`Current Frame` :type Integer))
  (`self.is Animation Now` `Current Frame`
    (:`then`
      (`self.Set Current State` "NewEnumerator14")
      (`self.Stop Operator` 3))))

(event `Slap Event`
  (params (`Current Frame` :type Integer))
  (bind _output (`|GetArrayItem` (`self.Out Actors`)))
  (bind _capsulecomponent (`Character.CapsuleComponent` _output))
  (`self.is Animation Now` `Current Frame`
    (:`then`
      (`PrimitiveComponent.SetCollisionEnabled` _capsulecomponent "QueryAndPhysics")
      (`PrimitiveComponent.AddImpulse` _capsulecomponent (3000.0 0.0 0.0) "None" true)
      (`self.set Anim Default` 30))
    (:`else`
      (`PrimitiveComponent.SetCollisionEnabled` _capsulecomponent "NoCollision")
      (`SceneComponent.K2_SetWorldLocation` (`Actor.RootComponent` _output) (`SceneComponent.GetSocketLocation` (`self.Mesh`) "L_te") true false)
      (`PrimitiveComponent.SetSimulatePhysics` (`Character.CapsuleComponent` _output) true))))

(fn `Bind Input Actions`
  (bind _asplayer_controller (cast `PlayerController` (`self.GetController`)))
  (bind _returnvalue (pcsubsystem `EnhancedInputLocalPlayerSubsystem` _asplayer_controller))
  (`/Engine/EditorBlueprintResources/StandardMacros.IsValid` _returnvalue
    (:`Is Valid`
      (`EnhancedInputSubsystemInterface.AddMappingContext` _returnvalue "/Game/DefaultSetting/IMC_Default.IMC_Default" 0 (struct)))))

(fn `Bind WBP`
  (bind _aswbp_sample_gage_v1 (cast `/Game/member/Okajima/wbp/WBP_SampleGageV1` (`WidgetComponent.GetUserWidgetObject` (`self.Widget`))))
  (bind _output_get (set `self.HP Gage` _aswbp_sample_gage_v1))
  (`/Game/member/Okajima/wbp/WBP_SampleGageV1.UpdateHealthProgress` _output_get (/ (`self.HP`) (`self.MAXHP`))))

(fn `Set Current State`
  (params (`Next State` :type "/Game/member/Okajima/PlayerSource/BP_PlayerBaseAnimState Enum" :default "NewEnumerator0"))
  (set `self.Current State` `Next State`)
  (set `self.Anim Frame` 0)
  (switch `/Game/member/Okajima/PlayerSource/BP_PlayerBaseAnimState` `Next State`
    (:`NewEnumerator0`
      (set `self.Finish Anim Frame` 0))
    (:`NewEnumerator11`
      (set `self.Finish Anim Frame` 50))
    (:`NewEnumerator12`
      (set `self.Finish Anim Frame` 48))
    (:`NewEnumerator13`
      (set `self.Finish Anim Frame` 26))
    (:`NewEnumerator14`
      (set `self.Finish Anim Frame` 43))
    (:`NewEnumerator17`
      (set `self.Finish Anim Frame` 36))
    (:`NewEnumerator18`
      (set `self.Finish Anim Frame` 36))
    (:`NewEnumerator19`
      (set `self.Finish Anim Frame` 20))))

(fn `Update All State`
  (params (`Current Frame` :type Integer) (`Current State` :type "/Game/member/Okajima/PlayerSource/BP_PlayerBaseAnimState Enum" :default "NewEnumerator0"))
  (switch `/Game/member/Okajima/PlayerSource/BP_PlayerBaseAnimState` `Current State`
    (:`NewEnumerator11`
      (`self.Moment Attack Event` `Current Frame`))
    (:`NewEnumerator12`
      (`self.Success Event` `Current Frame`))
    (:`NewEnumerator13`
      (`self.Avoidance Event` `Current Frame`))
    (:`NewEnumerator14`
      (`self.Slap Event` `Current Frame`))
    (:`NewEnumerator18`
      (`self.FAILED Event` `Current Frame`))
    (:`NewEnumerator19`
      (`self.Grabbed Event` `Current Frame`))))

(fn `UserConstructionScript`
  (set `self.HP` (`self.MAXHP`)))