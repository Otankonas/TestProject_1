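; Player character base that handles Enhanced Input movement, jumping, attack combos, avoidance, lock-on and grab-related actions.
; A state machine updated on Tick times each action with per-state frame counts, counted in ticks rather than by animation callbacks.
; Lock-on picks the nearest GrabBaseV1 actor, cycles targets on press and releases on hold.
; Timeline-driven runs dash sideways or toward the locked target, where GrabChance switches input to grab attack and avoidance.
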(event `self.ReceiveBeginPlay`
  (`|ExecutionSequence`
    (:`then_0`
      (`self.Bind Input Actions`))
    (:`then_1`
      (`self.Init Set All Grab Actors`))
    (:`then_2`
      (set `self.CurrentState` "NewEnumerator0"))))

(event `self.ReceiveTick`
  (params (DeltaSeconds :type "Float (single-precision)"))
  (bind _animframecount (`self.AnimFrameCount`))
  (`|ExecutionSequence`
    (:`then_0`
      (`self.Update All State` _animframecount (`self.CurrentState`))
      (`/Engine/EditorBlueprintResources/StandardMacros.IncrementInt` _animframecount))
    (:`then_1`
      (`self.is LockOn`
        (:`then`
          (`self.Turn Toward The Actor`))))))

(event `self.ReceiveAnyDamage`
  (params (Damage :type "Float (single-precision)") (DamageType :type "DamageType Object Reference") (InstigatedBy :type "Controller Object Reference") (DamageCauser :type "Actor Object Reference"))
  (`self.is Avoidance`
    (:`else`
      (`self.Set Current State` "NewEnumerator16")
      (set `self.Grab Chance` false))))

(event `EnhancedInput|/Game/DefaultSetting/inputAction/IA_Jump`
  (params (ActionValue :type Boolean) (ElapsedSeconds :type "Float (double-precision)") (TriggeredSeconds :type "Float (double-precision)") (InputAction :type "InputAction Object Reference" :default "/Game/DefaultSetting/inputAction/IA_Jump.IA_Jump"))
  ;[1 0.02677 0] Input Action -Jump-
  (:`Started`
    (`self.is Grab Chance`
      (:`else`
        (switch `/Game/member/Okajima/PlayerSource/BP_PlayerBaseAnimState` (`self.CurrentState`)
          (:`NewEnumerator0`
            (`self.Jump`)
            (`self.Set Current State` "NewEnumerator7"))
          (:`NewEnumerator1`
            (`self.Jump`)
            (`self.Set Current State` "NewEnumerator7"))))))
  (:`Completed`
    (`self.StopJumping`)))

(event `EnhancedInput|/Game/DefaultSetting/inputAction/IA_Move`
  (params (ActionValue :type "Vector2D Structure") (ElapsedSeconds :type "Float (double-precision)") (TriggeredSeconds :type "Float (double-precision)") (InputAction :type "InputAction Object Reference" :default "/Game/DefaultSetting/inputAction/IA_Move.IA_Move"))
  (bind _degree (`self.Get Angle From Zero` (`self.Get Controller Value Y`) (`self.Get Controller Value X`)))
  ;[1 0.3505 0.0776] Input Action -Move-
  (:`Triggered`
    (`|ExecutionSequence`
      (:`then_0`
        (`KismetArrayLibrary.Array_Set` (`self.Controller Trigger Value XY`) 0 ActionValue_X)
        (`KismetArrayLibrary.Array_Set` (`self.Controller Trigger Value XY`) 1 ActionValue_Y))
      (:`then_1`
        (`self.is Grab Chance`
          (:`else`
            (switch `/Game/member/Okajima/PlayerSource/BP_PlayerBaseAnimState` (`self.CurrentState`)
              (:`NewEnumerator0`
                _)
              (:`NewEnumerator1`
                _))
            (`self.AddMovementInput` (`self.Get Controller Rightward Vector`) (`self.Get Controller Value X`))
            (`self.AddMovementInput` (`self.Get Controller Forward Vector`) (`self.Get Controller Value Y`))
            (`SceneComponent.K2_SetWorldRotation` (`self.Mesh`) (`KismetMathLibrary.MakeRotator` 0.0 0.0 (+ _degree -45.0)) false false)
            (`|ExecutionSequence`
              (:`then_0`
                (`self.Set Current State` "NewEnumerator1"))
              (:`then_1`
                (`SceneComponent.K2_SetWorldRotation` (`self.GA1C`) (`KismetMathLibrary.MakeRotator` 0.0 0.0 _degree) false false)
                (`SceneComponent.K2_SetWorldRotation` (`self.GA2C`) (`KismetMathLibrary.MakeRotator` 0.0 0.0 _degree) false false)
                (`SceneComponent.K2_SetWorldRotation` (`self.GA3C`) (`KismetMathLibrary.MakeRotator` 0.0 0.0 _degree) false false)
                (`SceneComponent.K2_SetWorldRotation` (`self.AAC`) (`KismetMathLibrary.MakeRotator` 0.0 0.0 _degree) false false)))))))))

(event `EnhancedInput|/Game/DefaultSetting/inputAction/IA_LockOn`
  (params (ActionValue :type Boolean) (ElapsedSeconds :type "Float (double-precision)") (TriggeredSeconds :type "Float (double-precision)") (InputAction :type "InputAction Object Reference" :default "/Game/DefaultSetting/inputAction/IA_LockOn.IA_LockOn"))
  ;[1 0.9061 0.1159] Input Action -LockOn-
  (:`Triggered`
    (`self.is Grab Chance`
      (:`else`
        (`self.is LockOn`
          (:`then`
            (`self.is Valid Grab Actors`
              (:`Is Valid`
                (bind _result (`/Engine/EditorBlueprintResources/StandardMacros.IncrementInt` (`self.LockOn Release Frame`))
                  (:`  `
                    (if (> (`KismetMathLibrary.Conv_IntToDouble` _result) (`self.Get World Delta Frame`))
                      (set `self.LockOn Release Frame` 0)
                      (set `self.LockOn` false)))))))))))
  (:`Started`
    (`self.is Grab Chance`
      (:`else`
        (`self.is LockOn`
          (:`then`
            (`/Engine/EditorBlueprintResources/StandardMacros.IncrementInt` (`self.LockOn Index`)
              (:`  `
                (if (> (`self.LockOn Index`) (- (`KismetArrayLibrary.Array_Length` (`self.Grab Actors`)) 1))
                  (set `self.LockOn Index` 0)))))
          (:`else`
            (switch `/Game/member/Okajima/PlayerSource/BP_PlayerBaseAnimState` (`self.CurrentState`)
              (:`NewEnumerator0`
                _)
              (:`NewEnumerator1`
                _))
            (`self.is Valid Grab Actors`
              (:`Is Valid`
                (for (_array_element _array_index) (`self.Grab Actors`)
                  (bind _distance (`self.Get Grab Actor Distance` _array_element))
                  (if (> (`self.LockOn Distance`) _distance)
                    (set `self.LockOn Distance` _distance)
                    (set `self.LockOn Index` _array_index)))
                (`self.Turn Toward The Actor`)
                (set `self.LockOn` true))))))))
  (:`Completed`
    (set `self.LockOn Release Frame` 0)))

(event `EnhancedInput|/Game/DefaultSetting/inputAction/IA_Run`
  (params (ActionValue :type Boolean) (ElapsedSeconds :type "Float (double-precision)") (TriggeredSeconds :type "Float (double-precision)") (InputAction :type "InputAction Object Reference" :default "/Game/DefaultSetting/inputAction/IA_Run.IA_Run"))
  ;[0.5405 1 0.1075] Input Action -Run-
  (:`Started`
    (`self.is Grab`
      (:`else`
        (`self.is Grab Chance`
          (:`else`
            (`self.is LockOn`
              (:`then`
                (`self.is Valid Grab Actors`
                  (:`Is Valid`
                    (`self.is LockOn Run`
                      (:`else`
                        (`KismetArrayLibrary.Array_Set` (`self.Run Location`) 0 (`self.K2_GetActorLocation`))
                        (set `self.Grab Actor` (`|GetArrayItem` (`self.Grab Actors`) (`self.LockOn Index`)))
                        (`KismetArrayLibrary.Array_Set` (`self.Run Location`) 1 (`self.K2_GetActorLocation` (`self.Grab Actor`)))
                        (set `self.LockOn Run` true)
                        (`self.Set Current State` "NewEnumerator10")
                        (`TimelineComponent.PlayFromStart` (`self.LockOn Run Timeline`)))))))
              (:`else`
                (`self.is Normal Run`
                  (:`else`
                    (`KismetArrayLibrary.Array_Set` (`self.Run Location`) 0 (`self.K2_GetActorLocation`))
                    (`/Engine/EditorBlueprintResources/StandardMacros.CompareFloat` (`self.Get Controller Value X`)
                      (:`>`
                        (`KismetArrayLibrary.Array_Set` (`self.Run Location`) 1 (+ (`self.K2_GetActorLocation`) (0.0 500.0 0.0)))
                        (set `self.Normal Run` true)
                        (`self.Set Current State` "NewEnumerator10")
                        (`TimelineComponent.PlayFromStart` (`self.Normal Run Timeline`)))
                      (:`<`
                        (`KismetArrayLibrary.Array_Set` (`self.Run Location`) 1 (+ (`self.K2_GetActorLocation`) (0.0 -500.0 0.0)))
                        (set `self.Normal Run` true)
                        (`self.Set Current State` "NewEnumerator10")
                        (`TimelineComponent.PlayFromStart` (`self.Normal Run Timeline`))))))))))))))

(event `EnhancedInput|/Game/DefaultSetting/inputAction/IA_Attack`
  (params (ActionValue :type Boolean) (ElapsedSeconds :type "Float (double-precision)") (TriggeredSeconds :type "Float (double-precision)") (InputAction :type "InputAction Object Reference" :default "/Game/DefaultSetting/inputAction/IA_Attack.IA_Attack"))
  (bind _currentstate (`self.CurrentState`))
  ;[0 1 0.2243] Input Action -Attack-
  (:`Started`
    (`self.is Grab Chance`
      (:`then`
        ;[1 0 0.04229] - Not Use - Input Action -Grab Attack-
        (if (and (`|EnumInequality` _currentstate "NewEnumerator3") (`|EnumInequality` _currentstate "NewEnumerator16"))
          (`self.Set Current State` "NewEnumerator11")))
      (:`else`
        (switch `/Game/member/Okajima/PlayerSource/BP_PlayerBaseAnimState` (`self.CurrentState`)
          (:`NewEnumerator0`
            (`self.Set Current State` "NewEnumerator3" :!label _label))
          (:`NewEnumerator1`
            (goto _label))
          (:`NewEnumerator7`
            (`self.Set Current State` "NewEnumerator6" :!label _label_2))
          (:`NewEnumerator8`
            (goto _label_2)))))))

(event `EnhancedInput|/Game/DefaultSetting/inputAction/IA_GrabAttack`
  (params (ActionValue :type Boolean) (ElapsedSeconds :type "Float (double-precision)") (TriggeredSeconds :type "Float (double-precision)") (InputAction :type "InputAction Object Reference" :default "/Game/DefaultSetting/inputAction/IA_GrabAttack.IA_GrabAttack"))
  ;[1 0 0.04229] - Not Use - Input Action -Grab Attack-
)

(event `EnhancedInput|/Game/DefaultSetting/inputAction/IA_Avoidance`
  (params (ActionValue :type Boolean) (ElapsedSeconds :type "Float (double-precision)") (TriggeredSeconds :type "Float (double-precision)") (InputAction :type "InputAction Object Reference" :default "/Game/DefaultSetting/inputAction/IA_Avoidance.IA_Avoidance"))
  (bind _currentstate (`self.CurrentState`))
  ;[0 0.9218 1] Input Action -Avoidance-
  (:`Started`
    (`self.is Grab Chance`
      (:`then`
        (if (and (`|EnumInequality` _currentstate "NewEnumerator13") (`|EnumInequality` _currentstate "NewEnumerator16"))
          (`self.Set Current State` "NewEnumerator13")
          (set `self.Avoidance` true))))))

(event `EnhancedInput|/Game/DefaultSetting/inputAction/IA_Slap`
  (params (ActionValue :type Boolean) (ElapsedSeconds :type "Float (double-precision)") (TriggeredSeconds :type "Float (double-precision)") (InputAction :type "InputAction Object Reference" :default "/Game/DefaultSetting/inputAction/IA_Slap.IA_Slap"))
  ;[0 0.2763 1] Input Action -Slap-
  (:`Started`
    (`self.is Grab`
      (:`then`
        (`self.Set Current State` "NewEnumerator14")))))

(event `EnhancedInput|/Game/DefaultSetting/inputAction/IA_Throw`
  (params (ActionValue :type Boolean) (ElapsedSeconds :type "Float (double-precision)") (TriggeredSeconds :type "Float (double-precision)") (InputAction :type "InputAction Object Reference" :default "/Game/DefaultSetting/inputAction/IA_Throw.IA_Throw"))
  ;[0.5238 0 1] Input Action -Throw-
  (:`Started`
    (`self.is Grab`
      (:`then`
        (`self.is LockOn`
          (:`then`
            (`self.Set Current State` "NewEnumerator15")))))))

(event `Jump Event`
  (params (CurrentFrame :type Integer))
  (if (`self.is Falling`)
    (if (>= CurrentFrame (`self.FinishAnimFrameCount`))
      (`self.Set Current State` "NewEnumerator8"))
    (else
      (`self.Set Current State` "NewEnumerator9"))))

(event `Fall Event`
  (if (not (`self.is Falling`))
    (`self.Set Current State` "NewEnumerator9")))

(event `Land Event`
  (params (`Current Frame` :type Integer))
  (if (>= `Current Frame` (`self.FinishAnimFrameCount`))
    (`self.Set Current State` "NewEnumerator0")))

(event `Stop Event`
  (params (CurrentFrame :type Integer))
  (if (>= CurrentFrame (`self.FinishAnimFrameCount`))
    (`self.Set Current State` "NewEnumerator0")))

(event `Move Event`
  (if (`self.is Falling`)
    (`self.Set Current State` "NewEnumerator8")
    (elif (`self.is Velocity` 1.0 1.0)
      (`self.Set Current State` "NewEnumerator0"))))

(event `GAttack1 Event`
  (params (`Current Frame` :type Integer))
  (bind _finishanimframecount (`self.FinishAnimFrameCount`))
  (`|ExecutionSequence`
    (:`then_0`
      (if (>= `Current Frame` _finishanimframecount)
        (if (>= `Current Frame` (+ _finishanimframecount 10))
          (`self.Set Current State` "NewEnumerator0")
          (elif (`|GetInputActionValue`)
            (`self.Set Current State` "NewEnumerator4")))))))

(event `GAttack2 Event`
  (params (`Current Frame` :type Integer))
  (bind _finishanimframecount (`self.FinishAnimFrameCount`))
  (if (>= `Current Frame` _finishanimframecount)
    (if (>= `Current Frame` (+ _finishanimframecount 10))
      (`self.Set Current State` "NewEnumerator0")
      (elif (`|GetInputActionValue`)
        (`self.Set Current State` "NewEnumerator5")))))

(event `GAttack3 Event`
  (params (`Current Frame` :type Integer))
  (if (>= `Current Frame` (`self.FinishAnimFrameCount`))
    (`self.Set Current State` "NewEnumerator0")))

(event `AAttack Event`
  (params (`Current Frame` :type Integer))
  (if (>= `Current Frame` (`self.FinishAnimFrameCount`))
    (`self.Set Current State` "NewEnumerator0")))

(event `GrabAttack Event`
  (params (`Current Frame` :type Integer))
  ;[1 0.003152 0] 掴み攻撃　条件あとで追加せんなんとこ
  (if (>= `Current Frame` (`self.FinishAnimFrameCount`))
    (set `self.Grab Failed` false)
    (`self.Set Current State` "NewEnumerator0")
    (elif (>= `Current Frame` 14)
      (set `self.Grab Failed` true))))

(event `Avoidance Event`
  (params (`Current Frame` :type Integer))
  ;[1 1 1] 無敵判定もつくらんなん
  (if (>= `Current Frame` (`self.FinishAnimFrameCount`))
    (`self.Set Current State` "NewEnumerator0")
    (set `self.Avoidance` false)))

(event `Damage Event`
  (params (`Current Frame` :type Integer))
  (if (>= `Current Frame` (`self.FinishAnimFrameCount`))
    (`self.Set Current State` "NewEnumerator0")))

(event `Slap Event`
  (params (`Current Frame` :type Integer))
  (if (>= `Current Frame` (`self.FinishAnimFrameCount`))
    (`self.Set Current State` "NewEnumerator0")))

(event `Throw Event`
  (params (`Current Frame` :type Integer))
  (if (>= `Current Frame` (`self.FinishAnimFrameCount`))
    (`self.Set Current State` "NewEnumerator0")))

(fn `Bind Input Actions`
  (bind _asplayer_controller (cast `PlayerController` (`self.GetController`)))
  (bind _returnvalue (pcsubsystem `EnhancedInputLocalPlayerSubsystem` _asplayer_controller))
  (`/Engine/EditorBlueprintResources/StandardMacros.IsValid` _returnvalue
    (:`Is Valid`
      (`EnhancedInputSubsystemInterface.AddMappingContext` _returnvalue "/Game/DefaultSetting/IMC_Default.IMC_Default" 0 (struct))
      (`KismetSystemLibrary.PrintString` "Completed Bind Input Actions!!!"))
    (:`Is Not Valid`
      (`KismetSystemLibrary.PrintString` "Failed Bind Input Actions!!!" true true (struct :`R` 1.0 :`G` 0.026892 :`A` 1.0)))))

(fn `Create Prediction Path`
  (`|ExecutionSequence`))

(fn `Init Set All Grab Actors`
  (bind _outactors (`GameplayStatics.GetAllActorsOfClass` "/Game/member/Okajima/EnemySource/GrabBaseV1.GrabBaseV1_C"))
  (set `self.Grab Actors` _outactors)
  (set `self.Grab Actor` null)
  (`KismetSystemLibrary.PrintString` "Completed Set Grab Actors!!!"))

(fn `Set Current State`
  (params (`Next State` :type "/Game/member/Okajima/PlayerSource/BP_PlayerBaseAnimState Enum" :default "NewEnumerator0"))
  (set `self.CurrentState` `Next State`)
  (set `self.AnimFrameCount` 0)
  (switch `/Game/member/Okajima/PlayerSource/BP_PlayerBaseAnimState` `Next State`
    (:`NewEnumerator0`
      (set `self.FinishAnimFrameCount` 0 :!label _label))
    (:`NewEnumerator1`
      (goto _label))
    (:`NewEnumerator2`
      (set `self.FinishAnimFrameCount` 21))
    (:`NewEnumerator3`
      (set `self.FinishAnimFrameCount` 5 :!label _label_2))
    (:`NewEnumerator4`
      (goto _label_2))
    (:`NewEnumerator5`
      (set `self.FinishAnimFrameCount` 14))
    (:`NewEnumerator6`
      (set `self.FinishAnimFrameCount` 16))
    (:`NewEnumerator7`
      (set `self.FinishAnimFrameCount` 12))
    (:`NewEnumerator8`
      (goto _label))
    (:`NewEnumerator9`
      (set `self.FinishAnimFrameCount` 7))
    (:`NewEnumerator10`
      (set `self.FinishAnimFrameCount` 50))
    (:`NewEnumerator11`
      (set `self.FinishAnimFrameCount` 40))
    (:`NewEnumerator12`
      (set `self.FinishAnimFrameCount` 48))
    (:`NewEnumerator13`
      (set `self.FinishAnimFrameCount` 26))
    (:`NewEnumerator14`
      (set `self.FinishAnimFrameCount` 43))
    (:`NewEnumerator15`
      (set `self.FinishAnimFrameCount` 43))
    (:`NewEnumerator16`
      (set `self.FinishAnimFrameCount` 42))
    (:`NewEnumerator17`
      (set `self.FinishAnimFrameCount` 17))))

(fn `Turn Toward The Actor`
  (bind (_returnvalue_roll _returnvalue_pitch _returnvalue_yaw) (`KismetMathLibrary.BreakRotator` (`KismetMathLibrary.FindLookAtRotation` (`self.K2_GetActorLocation`) (`self.K2_GetActorLocation` (`|GetArrayItem` (`self.Grab Actors`) (`self.LockOn Index`))))))
  (`SceneComponent.K2_SetWorldRotation` (`self.Mesh`) (`KismetMathLibrary.MakeRotator` 0.0 0.0 (+ _returnvalue_yaw -90.0)) false false))

(fn `Update All State`
  (params (CurrentFrame :type Integer) (CurrentState :type "/Game/member/Okajima/PlayerSource/BP_PlayerBaseAnimState Enum" :default "NewEnumerator0"))
  (switch `/Game/member/Okajima/PlayerSource/BP_PlayerBaseAnimState` CurrentState
    (:`NewEnumerator1`
      (`self.Move Event`))
    (:`NewEnumerator2`
      (`self.Stop Event` CurrentFrame))
    (:`NewEnumerator3`
      (`self.GAttack1 Event` CurrentFrame))
    (:`NewEnumerator4`
      (`self.GAttack2 Event` CurrentFrame))
    (:`NewEnumerator5`
      (`self.GAttack3 Event` CurrentFrame))
    (:`NewEnumerator6`
      (`self.AAttack Event` CurrentFrame))
    (:`NewEnumerator7`
      (`self.Jump Event` CurrentFrame))
    (:`NewEnumerator8`
      (`self.Fall Event`))
    (:`NewEnumerator9`
      (`self.Land Event` CurrentFrame))
    (:`NewEnumerator11`
      (`self.GrabAttack Event` CurrentFrame))
    (:`NewEnumerator13`
      (`self.Avoidance Event` CurrentFrame))
    (:`NewEnumerator14`
      (`self.Slap Event` CurrentFrame))
    (:`NewEnumerator15`
      (`self.Throw Event` CurrentFrame))
    (:`NewEnumerator16`
      (`self.Damage Event` CurrentFrame))))

(fn `Update Grab Chance Battle`)

(fn `UserConstructionScript`)