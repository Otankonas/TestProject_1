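; Camera actor that makes itself the first player's view target on BeginPlay, built for side-view player following.
; Helper functions track the pawn's Y, optionally Z for jumps, at a fixed X, and ramp an alpha for attack-driven spring-arm zoom.
; That follow logic and the boss-room lerp are disconnected, leaving Tick empty.
; A test event moves and rotates the Scene component to hard-coded values.
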(event `self.ReceiveBeginPlay`
  ;[1 1 1] 初期配置
  (`PlayerController.SetViewTargetWithBlend` (`GameplayStatics.GetPlayerController` 0) self 0.0 "VTBlend_Linear" 0.0 false))

(event `test Next Location`
  (bind _scene (`self.Scene`))
  (`SceneComponent.K2_SetWorldLocation` _scene (250.0 160.0 -10.0) true false)
  (`SceneComponent.K2_SetWorldRotation` _scene (struct :`Yaw` -140.0) false false))

(event `self.ReceiveTick`
  (params (DeltaSeconds :type "Float (single-precision)")))

(fn `CameraLengeLerp`
  (params (IsAtack :type Boolean) (NewParam :type "Float (double-precision)"))
  (bind _targetlenlerp (`self.TargetLenLerp`))
  (if IsAtack
    (bind `_加算結果` (`self.α値加算` _targetlenlerp NewParam))
    (set `self.TargetLenLerp` `_加算結果`)
    (else
      (bind `_減算結果` (`self.α値減算` _targetlenlerp NewParam))
      (set `self.TargetLenLerp` `_減算結果`))))

(fn `CameraPosXLerp`
  (params (NewParam :type Boolean))
  (bind _camerapos_x (`KismetMathLibrary.BreakVector` (`self.CameraPos`)))
  (bind _returnvalue_x (`KismetMathLibrary.BreakVector` (`self.K2_GetActorLocation` (`self.GetPlayer`))))
  (if NewParam
    (`self.K2_SetActorLocation` (`KismetMathLibrary.MakeVector` (`KismetMathLibrary.Lerp` _camerapos_x (- _returnvalue_x 500.0) (`self.TargetLenLerp`))))))

(fn `SetLocation`
  (params (NewParam :type "Vector Structure"))
  (bind _output_get (set `self.CameraPos` (`KismetMathLibrary.MakeVector` (`self.TargetLen`) NewParam_Y (`self.LocationZ`))))
  (`self.K2_SetActorLocation` _output_get true))

(fn `SetLocation2D`
  (params (self2 :type "Vector Structure"))
  (bind _output_get (set `self.LocationZ` (+ self2_Z 120.0)))
  (bind _output_get_2 (set `self.CameraPos` (`KismetMathLibrary.MakeVector` (`self.TargetLen`) self2_Y _output_get)))
  (`self.K2_SetActorLocation` _output_get_2 true))

(fn `SetLocationFirst`
  (params (length :type "Float (double-precision)") (PlayerPos :type "Vector Structure"))
  (bind _output_get (set `self.LocationZ` PlayerPos_Z))
  (bind _output_get_2 (set `self.TargetLen` (- PlayerPos_X length)))
  (bind _output_get_3 (set `self.CameraPos` (`KismetMathLibrary.MakeVector` _output_get_2 PlayerPos_Y _output_get)))
  (`self.K2_SetActorLocation` _output_get_3 true))

(fn `UserConstructionScript`)

(fn `α値加算`
  (params (`加算する変数` :type "Float (double-precision)") (`加算量` :type "Float (double-precision)"))
  (returns (`加算結果` :type "Float (double-precision)"))
  (if (< `加算する変数` 1.0)
    (return (+ `加算する変数` `加算量`))
    (else
      (return `加算する変数`))))

(fn `α値減算`
  (params (`減算する変数` :type "Float (double-precision)") (`減算量` :type "Float (double-precision)"))
  (returns (`減算結果` :type "Float (double-precision)"))
  (if (> `減算する変数` 0.0)
    (return (- `減算する変数` `減算量`))
    (else
      (return `減算する変数`))))