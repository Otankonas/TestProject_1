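; Grabbable enemy-style actor that runs a pull tug-of-war with the player through a Tick-driven state machine.
; In grab states it faces the player, picks a random cardinal pull direction, then after an interval spawns staggered afterimages along it.
; When the last afterimage is destroyed, it briefly jerks that way if the player's pull is incorrect, then repeats.
; Damage drains a self-recovering widget gauge; emptying it breaks the grab.
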(event `self.ReceiveBeginPlay`
  (`|ExecutionSequence`
    (:`then_0`
      (bind _asbp_player_base_v1 (cast `/Game/member/Okajima/bp/BP_PlayerBaseV1` (`GameplayStatics.GetPlayerPawn` 0)))
      (set `self.CurrentPlayer` _asbp_player_base_v1))
    (:`then_1`
      (bind _aswbp_sample_gage_v1 (cast `/Game/member/Okajima/wbp/WBP_SampleGageV1` (`WidgetComponent.GetUserWidgetObject` (`self.Widget`))))
      (set `self.SampleGage1` _aswbp_sample_gage_v1))
    (:`then_2`
      (set `self.CurrentState` "NewEnumerator0"))))

(event `self.ReceiveAnyDamage`
  (params (Damage :type "Float (single-precision)") (DamageType :type "DamageType Object Reference") (InstigatedBy :type "Controller Object Reference") (DamageCauser :type "Actor Object Reference"))
  (bind _output_get (set `self.CurrentGageValue` (`KismetMathLibrary.FMax` (- (`self.CurrentGageValue`) Damage))))
  (if (`KismetMathLibrary.NearlyEqual_FloatFloat` _output_get)
    (`/Game/member/Okajima/wbp/WBP_SampleGageV1.UpdateHealthProgress` (`self.SampleGage1`) 0.0)
    (set `self.Break` true)
    (else
      (`/Game/member/Okajima/wbp/WBP_SampleGageV1.UpdateHealthProgress` (`self.SampleGage1`) (/ (`self.CurrentGageValue`) (`self.MaxGageValue`))))))

(event `self.ReceiveTick`
  (params (DeltaSeconds :type "Float (single-precision)"))
  (bind _returnvalue (`self.GetTransform`))
  (bind _returnvalue_2 (`self.GetTransform`))
  (bind _returnvalue_3 (`self.GetTransform`))
  (bind (_returnvalue_roll _returnvalue_pitch _returnvalue_yaw) (`KismetMathLibrary.BreakRotator` (`SceneComponent.K2_GetComponentRotation` (`self.Mesh`))))
  (bind (_returnvalue_roll_2 _returnvalue_pitch_2 _returnvalue_yaw_2) (`KismetMathLibrary.BreakRotator` (`SceneComponent.K2_GetComponentRotation` (`self.Mesh`))))
  (bind (_returnvalue_roll_3 _returnvalue_pitch_3 _returnvalue_yaw_3) (`KismetMathLibrary.BreakRotator` (`SceneComponent.K2_GetComponentRotation` (`self.Mesh`))))
  (switch `/Game/member/Okajima/state/GrabBaseV1State` (`self.CurrentState`)
    (:`NewEnumerator1`
      (`self.Function GBReady`))
    (:`NewEnumerator2`
      (`self.Function GB`))
    (:`NewEnumerator3`
      (`|ExecutionSequence`
        (:`then_0`
          (`self.Function GBAttack`))
        (:`then_1`
          (if (`self.AttackAfterEffectSpawflg`)
            (`/Engine/EditorBlueprintResources/StandardMacros.DoOnce` false :!label _label
              (:`Completed`
                (bind _degree (`self.Get Degree` (`self.PullingYValue`) (`self.PullingXValue`)))
                (`|SpawnActorFromClass` "/Game/member/Okajima/bp/BP_GrabActorT1V1AfterEffect.BP_GrabActorT1V1AfterEffect_C" (`KismetMathLibrary.MakeTransform` (`KismetMathLibrary.MakeVector` (+ (* (`KismetMathLibrary.DegCos` _degree) 10.0) (.x (.location _returnvalue))) (+ (* (`KismetMathLibrary.DegSin` _degree) 10.0) (.y (.location _returnvalue))) (.z (.location _returnvalue))) (`KismetMathLibrary.MakeRotator` _returnvalue_roll _returnvalue_pitch (+ _returnvalue_yaw 90.0)) (.scale _returnvalue)) "Undefined" "OverrideRootScale" null (struct) null)
                (`KismetSystemLibrary.Delay` 0.1)
                (bind _degree_2 (`self.Get Degree` (`self.PullingYValue`) (`self.PullingXValue`)))
                (`|SpawnActorFromClass` "/Game/member/Okajima/bp/BP_GrabActorT1V1AfterEffect.BP_GrabActorT1V1AfterEffect_C" (`KismetMathLibrary.MakeTransform` (`KismetMathLibrary.MakeVector` (+ (* (`KismetMathLibrary.DegCos` _degree_2) 20.0) (.x (.location _returnvalue_2))) (+ (* (`KismetMathLibrary.DegSin` _degree_2) 20.0) (.y (.location _returnvalue_2))) (.z (.location _returnvalue_2))) (`KismetMathLibrary.MakeRotator` _returnvalue_roll_2 _returnvalue_pitch_2 (+ _returnvalue_yaw_2 90.0)) (.scale _returnvalue_2)) "Undefined" "OverrideRootScale" null (struct) null)
                (`KismetSystemLibrary.Delay` 0.08)
                (bind _degree_3 (`self.Get Degree` (`self.PullingYValue`) (`self.PullingXValue`)))
                (bind _returnvalue_4 (`|SpawnActorFromClass` "/Game/member/Okajima/bp/BP_GrabActorT1V1AfterEffect.BP_GrabActorT1V1AfterEffect_C" (`KismetMathLibrary.MakeTransform` (`KismetMathLibrary.MakeVector` (+ (* (`KismetMathLibrary.DegCos` _degree_3) 30.0) (.x (.location _returnvalue_3))) (+ (* (`KismetMathLibrary.DegSin` _degree_3) 30.0) (.y (.location _returnvalue_3))) (.z (.location _returnvalue_3))) (`KismetMathLibrary.MakeRotator` _returnvalue_roll_3 _returnvalue_pitch_3 (+ _returnvalue_yaw_3 90.0)) (.scale _returnvalue_3)) "Undefined" "OverrideRootScale" null (struct) null))
                (set `self.LastAfterEffect` _returnvalue_4)))))
        (:`then_2`
          (bind _lastaftereffect (`self.LastAfterEffect`)
            (:`then`
              (add `self.OnDestroyed` _lastaftereffect (delegate `PullingAttack`)))
            (:`else`)))
        (:`then_3`
          (if (`self.Break`)
            (`self.Breaking`)
            (`KismetSystemLibrary.PrintString` "Hello")
            (elif (< (`self.CurrentGageValue`) (`self.MaxGageValue`))
              (set `self.CurrentGageValue` (+ (`self.CurrentGageValue`) (`self.GageRecoveryValue`)))
              (`/Game/member/Okajima/wbp/WBP_SampleGageV1.UpdateHealthProgress` (`self.SampleGage1`) (/ (`self.CurrentGageValue`) (`self.MaxGageValue`))))))))
    (:`NewEnumerator5`
      (`|ExecutionSequence`))
    (:`NewEnumerator6`
      (`KismetSystemLibrary.PrintString` "Hello"))))

(event `ResetAttack`
  (goto _label :!via `Reset`))

(event `PullingAttack` :!signature `self.OnDestroyed`
  (params (DestroyedActor :type "Actor Object Reference"))
  (bind (_returnvalue_x _returnvalue_y _returnvalue_z) (`KismetMathLibrary.BreakVector` (`self.K2_GetActorLocation`)))
  (bind _currentplayer (`self.CurrentPlayer`))
  (if (`/Game/member/Okajima/bp/BP_PlayerBaseV1.NotCorrectPulling` (`self.CurrentPlayer`))
    (bind _degree (`self.Get Degree` (`self.PullingYValue`) (`self.PullingXValue`)))
    (set `self.CurrentLocation` (`self.K2_GetActorLocation`))
    (`self.K2_SetActorLocation` (`KismetMathLibrary.MakeVector` (+ (* (`KismetMathLibrary.DegCos` _degree) 10.0) _returnvalue_x) (+ (* (`KismetMathLibrary.DegSin` _degree) 10.0) _returnvalue_y) _returnvalue_z))
    (`KismetSystemLibrary.Delay` 0.1)
    (`self.K2_SetActorLocation` (`self.CurrentLocation`))
    (else
      (`self.K2_SetActorLocation` (`self.CurrentLocation`))))
  (set `self.GBAttackCount` 0)
  (set `self.AttackAfterEffectSpawflg` false)
  (set `self.LastAfterEffect` null)
  (set `self.CurrentState` "NewEnumerator2")
  (set `/Game/member/Okajima/bp/BP_PlayerBaseV1.CorrectPulling` false _currentplayer)
  (set `/Game/member/Okajima/bp/BP_PlayerBaseV1.NotCorrectPulling` true _currentplayer)
  (`self.ResetAttack`))

(event `Breaking`
  (bind _currentplayer (`self.CurrentPlayer`))
  (set `self.AttackAfterEffectSpawflg` false)
  (set `self.LastAfterEffect` null)
  (set `self.GBAttackCount` 0)
  (set `/Game/member/Okajima/bp/BP_PlayerBaseV1.CorrectPulling` false _currentplayer)
  (set `/Game/member/Okajima/bp/BP_PlayerBaseV1.NotCorrectPulling` false _currentplayer)
  (set `/Game/member/Okajima/bp/BP_PlayerBaseV1.CurrentState` "NewEnumerator6" _currentplayer)
  (`KismetSystemLibrary.PrintString` "Reset!")
  (set `self.CurrentState` "NewEnumerator6")
  (`self.ResetAttack`))

(event `ThrowEnemy`
  (bind _currentplayer (`self.CurrentPlayer`))
  (set `self.Break` true)
  (set `self.AttackAfterEffectSpawflg` false)
  (set `self.LastAfterEffect` null)
  (set `self.GBAttackCount` 0)
  (set `self.CurrentState` "NewEnumerator5")
  (set `/Game/member/Okajima/bp/BP_PlayerBaseV1.CorrectPulling` false _currentplayer)
  (set `/Game/member/Okajima/bp/BP_PlayerBaseV1.NotCorrectPulling` false _currentplayer)
  (`KismetSystemLibrary.PrintString` "Reset!")
  (`self.ResetAttack`))

(fn `Function GB`
  (`|ExecutionSequence`
    (:`then_0`
      (`self.Function Lock On`)
      (set `self.CurrentLocation` (`self.K2_GetActorLocation`)))
    (:`then_1`
      (`self.Setting Pulling Direction`)
      (`KismetSystemLibrary.PrintString` "Setting Pulling Direction Value!" true true (struct :`R` 1.0 :`G` 0.02448 :`A` 1.0))
      (set `self.CurrentState` "NewEnumerator3"))))

(fn `Function GBAttack`
  (`|ExecutionSequence`
    (:`then_0`
      (`self.Function Lock On`))
    (:`then_1`
      (`/Engine/EditorBlueprintResources/StandardMacros.IncrementInt` (`self.GBAttackCount`)
        (:`  `
          (if (> (`KismetMathLibrary.Conv_IntToDouble` (`self.GBAttackCount`)) (/ (`self.AttackInterval`) (`GameplayStatics.GetWorldDeltaSeconds`)))
            (if (not (`self.AttackAfterEffectSpawflg`))
              (set `self.AttackAfterEffectSpawflg` true))))))))

(fn `Function GBReady`
  (`SceneComponent.K2_SetWorldRotation` (`self.Mesh`) (`KismetMathLibrary.MakeRotator` (.roll (`KismetMathLibrary.FindLookAtRotation` (`self.K2_GetActorLocation`) (`self.K2_GetActorLocation` (`self.CurrentPlayer`)))) (.pitch (`KismetMathLibrary.FindLookAtRotation` (`self.K2_GetActorLocation`) (`self.K2_GetActorLocation` (`self.CurrentPlayer`)))) (+ (.yaw (`KismetMathLibrary.FindLookAtRotation` (`self.K2_GetActorLocation`) (`self.K2_GetActorLocation` (`self.CurrentPlayer`)))) -90.0)) false false)
  (set `self.CurrentState` "NewEnumerator2"))

(fn `Function Lock On`
  (`SceneComponent.K2_SetWorldRotation` (`self.Mesh`) (`KismetMathLibrary.MakeRotator` (.roll (`KismetMathLibrary.FindLookAtRotation` (`self.K2_GetActorLocation`) (`self.K2_GetActorLocation` (`self.CurrentPlayer`)))) (.pitch (`KismetMathLibrary.FindLookAtRotation` (`self.K2_GetActorLocation`) (`self.K2_GetActorLocation` (`self.CurrentPlayer`)))) (+ (.yaw (`KismetMathLibrary.FindLookAtRotation` (`self.K2_GetActorLocation`) (`self.K2_GetActorLocation` (`self.CurrentPlayer`)))) -90.0)) false false))

(fn `Get Degree`
  (params (X :type "Float (double-precision)") (Y :type "Float (double-precision)"))
  (returns (Degree :type "Float (double-precision)"))
  (return (/ (* (`KismetMathLibrary.Atan2` (- Y 0.0) (- X 0.0)) 180.0) 3.14)))

(fn `Setting Pulling Direction`
  (bind _returnvalue (`KismetMathLibrary.RandomFloatInRange` -1.0 1.0))
  (bind _returnvalue_2 (`KismetMathLibrary.RandomFloatInRange` -1.0 1.0))
  (if (> _returnvalue_2 0.25)
    (set `self.PullingXValue` 1.0)
    (elif (> _returnvalue_2 -0.25)
      (set `self.PullingXValue` 0.0)
      (else
        (set `self.PullingXValue` -1.0))))
  (if (> _returnvalue 0.25)
    (set `self.PullingYValue` 1.0)
    (elif (> _returnvalue -0.25)
      (set `self.PullingYValue` 0.0)
      (else
        (set `self.PullingYValue` -1.0))))
  (`|ExecutionSequence`
    (:`then_0`
      (if (and (`KismetMathLibrary.NearlyEqual_FloatFloat` (`self.PullingXValue`)) (`KismetMathLibrary.NearlyEqual_FloatFloat` (`self.PullingYValue`)))
        (if (`KismetMathLibrary.RandomBool`)
          (set `self.PullingXValue` 1.0)
          (else
            (set `self.PullingYValue` 1.0)))))
    (:`then_1`
      (if (and (`KismetMathLibrary.NearlyEqual_FloatFloat` (`self.PullingXValue`) 1.0) (`KismetMathLibrary.NearlyEqual_FloatFloat` (`self.PullingYValue`) 1.0))
        (if (`KismetMathLibrary.RandomBool`)
          (set `self.PullingXValue` 0.0)
          (else
            (set `self.PullingYValue` 0.0)))))
    (:`then_2`
      (if (and (`KismetMathLibrary.NearlyEqual_FloatFloat` (`self.PullingXValue`) -1.0) (`KismetMathLibrary.NearlyEqual_FloatFloat` (`self.PullingYValue`) -1.0))
        (if (`KismetMathLibrary.RandomBool`)
          (set `self.PullingXValue` 0.0)
          (else
            (set `self.PullingYValue` 0.0)))))
    (:`then_3`
      (if (and (`KismetMathLibrary.NearlyEqual_FloatFloat` (`self.PullingXValue`) 1.0) (`KismetMathLibrary.NearlyEqual_FloatFloat` (`self.PullingYValue`) -1.0))
        (if (`KismetMathLibrary.RandomBool`)
          (set `self.PullingXValue` 0.0)
          (else
            (set `self.PullingYValue` 0.0)))))
    (:`then_4`
      (if (and (`KismetMathLibrary.NearlyEqual_FloatFloat` (`self.PullingXValue`) -1.0) (`KismetMathLibrary.NearlyEqual_FloatFloat` (`self.PullingYValue`) 1.0))
        (if (`KismetMathLibrary.RandomBool`)
          (set `self.PullingXValue` 0.0)
          (else
            (set `self.PullingYValue` 0.0)))))))

(fn `UserConstructionScript`
  (`parent.UserConstructionScript`)
  (set `self.CurrentGageValue` (`self.MaxGageValue`)))