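; BP_GrabBaseV2 is a base for grabbable objects, judging by its name, that carries a balance-point gauge and a direction widget.
; BeginPlay caches both widgets and the player pawn, hiding the direction indicator.
; Recovery and Damage set clamped targets; RecoveryGauge and DamageGauge, not called here, step balance toward them per call and update the gauge.
; Recovery clears BalanceBreak, but only unconnected damage logic sets it.
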(event `self.ReceiveBeginPlay`
  (`|ExecutionSequence`
    (:`then_0`
      (bind _aswbp_sample_gage_v1 (cast `/Game/member/Okajima/wbp/WBP_SampleGageV1` (`WidgetComponent.GetUserWidgetObject` (`self.Widget`))))
      (set `self.As WBP SampleGage1` _aswbp_sample_gage_v1)
      (bind _aswbp_sample_direction_v1 (cast `/Game/member/Okajima/wbp/WBP_SampleDirectionV1` (`WidgetComponent.GetUserWidgetObject` (`self.Widget1`))))
      (bind _output_get (set `self.As WBP Sample Direction V1` _aswbp_sample_direction_v1))
      (`/Game/member/Okajima/wbp/WBP_SampleDirectionV1.is not Show` _output_get))
    (:`then_1`
      (bind _asbp_player_base_v2 (cast `/Game/member/Okajima/Garbage/bp/BP_PlayerBaseV2` (`GameplayStatics.GetPlayerPawn` 0)))
      (set `self.As BP Player Base V2` _asbp_player_base_v2))))

(event `self.ReceiveAnyDamage`
  (params (Damage :type "Float (single-precision)") (DamageType :type "DamageType Object Reference") (InstigatedBy :type "Controller Object Reference") (DamageCauser :type "Actor Object Reference")))

(event `Event Recovery`
  (params (`Recovery Value` :type "Float (double-precision)"))
  (set `self.Recovery Value` (`KismetMathLibrary.FMin` (+ (`self.Current Balance Point`) `Recovery Value`) (`self.Max Balance Point`)))
  (set `self.Recovery` true)
  (set `self.Damage` false))

(event `Event Damage`
  (params (`Damage Value` :type "Float (double-precision)"))
  (set `self.Damage Value` (`KismetMathLibrary.FMax` (- (`self.Current Balance Point`) `Damage Value`)))
  (set `self.Damage` true)
  (set `self.Recovery` false))

(event `Recovery Gauge`
  (if (`self.Recovery`)
    (if (< (`self.Current Balance Point`) (`self.Recovery Value`))
      (set `self.Current Balance Point` (`KismetMathLibrary.FMin` (+ (`self.Current Balance Point`) 1.0) (`self.Max Balance Point`)))
      (`/Game/member/Okajima/wbp/WBP_SampleGageV1.UpdateHealthProgress` (`self.As WBP SampleGage1`) (/ (`self.Current Balance Point`) (`self.Max Balance Point`)))
      (set `self.Balance Break` false)
      (else
        (set `self.Recovery Value` -500.0)
        (set `self.Recovery` false)))))

(event `Damage Gauge`
  (if (`self.Damage`)
    (if (> (`self.Current Balance Point`) (`self.Damage Value`))
      (set `self.Current Balance Point` (`KismetMathLibrary.FMax` (- (`self.Current Balance Point`) 3.0)))
      (`/Game/member/Okajima/wbp/WBP_SampleGageV1.UpdateHealthProgress` (`self.As WBP SampleGage1`) (/ (`self.Current Balance Point`) (`self.Max Balance Point`)))
      (else
        (set `self.Damage Value` 500.0)
        (set `self.Damage` false)))))

(fn `UserConstructionScript`
  (set `self.Current Balance Point` (`self.Max Balance Point`)))