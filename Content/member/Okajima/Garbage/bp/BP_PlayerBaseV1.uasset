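; Player character Blueprint for lock-on, grab and tug-of-war play against grabbable actors.
; A Tick-driven state switch cycles lock-on targets gathered at BeginPlay, zooms the spring arm to the midpoint on a grab, then damages the target while stick input opposes its pull.
; Once the target breaks, it is held at the Sphere component.
; Spline-mesh throw-trajectory prediction and throwing logic exist but are not wired up.
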(event `EnhancedInput|/Game/DefaultSetting/inputAction/IA_LockOn`
  (params (ActionValue :type Boolean) (ElapsedSeconds :type "Float (double-precision)") (TriggeredSeconds :type "Float (double-precision)") (InputAction :type "InputAction Object Reference" :default "/Game/DefaultSetting/inputAction/IA_LockOn.IA_LockOn"))
  (bind _releaselockoncount (`self.ReleaseLockOnCount`))
  ;[1 1 1] ロックオン処理
  (:`Triggered`
    (switch `/Game/member/Okajima/state/PlayerBaseV1State` (`self.CurrentState`)
      (:`NewEnumerator1`
        (`/Engine/EditorBlueprintResources/StandardMacros.IncrementInt` _releaselockoncount
          (:`  `
            (if (> (`KismetMathLibrary.Conv_IntToDouble` _releaselockoncount) (/ 1.0 (`GameplayStatics.GetWorldDeltaSeconds`)))
              (set `self.ReleaseLockOnCount` 0)
              (set `self.CurrentState` "NewEnumerator0")))))))
  (:`Started`
    (switch `/Game/member/Okajima/state/PlayerBaseV1State` (`self.CurrentState`)
      (:`NewEnumerator0`
        (for (_array_element _array_index) (`self.Grab Items`)
          (bind _returnvalue (`KismetMathLibrary.Vector_Distance` (`self.K2_GetActorLocation` _array_element) (`self.K2_GetActorLocation`)))
          (if (> (`self.LockOnDistance`) _returnvalue)
            (set `self.LockOnDistance` _returnvalue)
            (set `self.LockOnIndex` _array_index)))
        (set `self.CurrentState` "NewEnumerator1")
        (`self.K2_SetActorRotation` (`KismetMathLibrary.FindLookAtRotation` (`self.K2_GetActorLocation`) (`self.K2_GetActorLocation` (`|GetArrayItem` (`self.Grab Items`) (`self.LockOnIndex`))))))
      (:`NewEnumerator1`
        (`/Engine/EditorBlueprintResources/StandardMacros.IncrementInt` (`self.LockOnIndex`)
          (:`  `
            (if (> (`self.LockOnIndex`) (- (`KismetArrayLibrary.Array_Length` (`self.Grab Items`)) 1))
              (set `self.LockOnIndex` 0))))))))

(event `EnhancedInput|/Game/DefaultSetting/inputAction/IA_Jump`
  (params (ActionValue :type Boolean) (ElapsedSeconds :type "Float (double-precision)") (TriggeredSeconds :type "Float (double-precision)") (InputAction :type "InputAction Object Reference" :default "/Game/DefaultSetting/inputAction/IA_Jump.IA_Jump"))
  ;[1 1 1] ジャンプ入力
  (:`Triggered`
    (`self.Jump`))
  (:`Completed`
    (`self.StopJumping`)))

(event `EnhancedInput|/Game/DefaultSetting/inputAction/IA_Move`
  (params (ActionValue :type "Vector2D Structure") (ElapsedSeconds :type "Float (double-precision)") (TriggeredSeconds :type "Float (double-precision)") (InputAction :type "InputAction Object Reference" :default "/Game/DefaultSetting/inputAction/IA_Move.IA_Move"))
  (bind (_returnvalue_roll _returnvalue_pitch _returnvalue_yaw) (`KismetMathLibrary.BreakRotator` (`self.GetControlRotation`)))
  (bind (_returnvalue_roll_2 _returnvalue_pitch_2 _returnvalue_yaw_2) (`KismetMathLibrary.BreakRotator` (`self.GetControlRotation`)))
  ;[1 1 1] スティック等、移動入力
  (:`Triggered`
    (`|ExecutionSequence`
      (:`then_0`
        (set `self.InputControllerXValue` ActionValue_X)
        (set `self.InputControllerYValue` ActionValue_Y)
        (switch `/Game/member/Okajima/state/PlayerBaseV1State` (`self.CurrentState`)
          (:`NewEnumerator0`
            _)
          (:`NewEnumerator1`
            _)
          (:`NewEnumerator6`
            _)
          (:`NewEnumerator7`
            _))
        (`self.AddMovementInput` (`KismetMathLibrary.GetRightVector` (`KismetMathLibrary.MakeRotator` _returnvalue_roll 0.0 _returnvalue_yaw)) (`self.InputControllerXValue`))
        (`self.AddMovementInput` (`KismetMathLibrary.GetForwardVector` (`KismetMathLibrary.MakeRotator` 0.0 0.0 _returnvalue_yaw_2)) (`self.InputControllerYValue`))
        (bind _degree (`self.Get Degree` (`self.InputControllerYValue`) (`self.InputControllerXValue`)))
        (`SceneComponent.K2_SetWorldRotation` (`self.Mesh`) (`KismetMathLibrary.MakeRotator` 0.0 0.0 (+ _degree -90.0)) false false))
      (:`then_1`
        (switch `/Game/member/Okajima/state/PlayerBaseV1State` (`self.CurrentState`)
          (:`NewEnumerator4`
            (set `self.Pulling` true))))))
  (:`Completed`
    (set `self.InputControllerXValue` 0.0)
    (set `self.InputControllerYValue` 0.0)
    (set `self.Pulling` false)))

(event `EnhancedInput|/Game/DefaultSetting/inputAction/IA_Grab`
  (params (ActionValue :type Boolean) (ElapsedSeconds :type "Float (double-precision)") (TriggeredSeconds :type "Float (double-precision)") (InputAction :type "InputAction Object Reference" :default "/Game/DefaultSetting/inputAction/IA_Grab.IA_Grab"))
  ;[1 1 1] つかむアクション
  (:`Started`
    (switch `/Game/member/Okajima/state/PlayerBaseV1State` (`self.CurrentState`)
      (:`NewEnumerator0`
        (if (< (`KismetMathLibrary.Vector_Distance` (`self.K2_GetActorLocation`) (`self.K2_GetActorLocation` (`|GetArrayItem` (`self.Grab Items`) (`self.LockOnIndex`)))) (`self.GrabDistance`))
          (set `self.CurrentState` "NewEnumerator3")
          (set `self.LockOnMoveFirstLocation` (`self.K2_GetActorLocation`))
          (bind _output_get (set `self.Grab Item` (`|GetArrayItem` (`self.Grab Items`) (`self.LockOnIndex`))))
          (`|ExecutionSequence`
            (:`then_0`
              (bind _asbp_grab_actor_t1v1 (cast `/Game/member/Okajima/Garbage/bp/BP_GrabActorT1V1` _output_get))
              (set `/Game/member/Okajima/Garbage/bp/BP_GrabActorT1V1.CurrentState` "NewEnumerator1" _asbp_grab_actor_t1v1)
              (set `/Game/member/Okajima/Garbage/bp/BP_GrabActorT1V1.Break` false _asbp_grab_actor_t1v1)))))
      (:`NewEnumerator1`
        (if (> (`KismetMathLibrary.Vector_Distance` (`self.K2_GetActorLocation`) (`self.K2_GetActorLocation` (`|GetArrayItem` (`self.Grab Items`) (`self.LockOnIndex`)))) (`self.GrabDistance`))
          (set `self.CurrentState` "NewEnumerator2")
          (set `self.LockOnMoveFirstLocation` (`self.K2_GetActorLocation`))
          (set `self.Grab Item` (`|GetArrayItem` (`self.Grab Items`) (`self.LockOnIndex`)))
          (`TimelineComponent.PlayFromStart` (`self.LockOnMove`))
          (else
            (set `self.CurrentState` "NewEnumerator3")
            (set `self.LockOnMoveFirstLocation` (`self.K2_GetActorLocation`))
            (bind _output_get_2 (set `self.Grab Item` (`|GetArrayItem` (`self.Grab Items`) (`self.LockOnIndex`))))
            (`|ExecutionSequence`
              (:`then_0`
                (bind _asbp_grab_actor_t1v1_2 (cast `/Game/member/Okajima/Garbage/bp/BP_GrabActorT1V1` _output_get_2))
                (set `/Game/member/Okajima/Garbage/bp/BP_GrabActorT1V1.CurrentState` "NewEnumerator1" _asbp_grab_actor_t1v1_2)
                (set `/Game/member/Okajima/Garbage/bp/BP_GrabActorT1V1.Break` false _asbp_grab_actor_t1v1_2)))))))))

(event `EnhancedInput|/Game/DefaultSetting/inputAction/IA_Throw`
  (params (ActionValue :type Boolean) (ElapsedSeconds :type "Float (double-precision)") (TriggeredSeconds :type "Float (double-precision)") (InputAction :type "InputAction Object Reference" :default "/Game/DefaultSetting/inputAction/IA_Throw.IA_Throw")))

(event `self.ReceiveBeginPlay`
  (`|ExecutionSequence`
    (:`then_0`
      ;[1 1 1] インプット処理バインド
      (bind _asplayer_controller (cast `PlayerController` (`self.GetController`)))
      (bind _returnvalue (pcsubsystem `EnhancedInputLocalPlayerSubsystem` _asplayer_controller))
      (`/Engine/EditorBlueprintResources/StandardMacros.IsValid` _returnvalue
        (:`Is Valid`
          (`EnhancedInputSubsystemInterface.AddMappingContext` _returnvalue "/Game/DefaultSetting/IMC_Default.IMC_Default" 0 (struct)))))
    (:`then_1`
      ;[1 1 1] シーン内にあるつかめるオブジェクトを取得
      (bind _outactors (`GameplayStatics.GetAllActorsOfClass` "/Game/member/Okajima/Garbage/bp/BP_GrabBaseV1.BP_GrabBaseV1_C"))
      (set `self.Grab Items` _outactors)
      (set `self.Grab Item` null))
    (:`then_2`
      ;[1 1 1] デフォルトのステートを設定
      (set `self.CurrentState` "NewEnumerator0")
      (set `self.CorrectPulling` false)
      (set `self.NotCorrectPulling` true))))

(event `Throw`)

(event `self.ReceiveTick`
  (params (DeltaSeconds :type "Float (single-precision)"))
  (`|ExecutionSequence`
    (:`then_0`
      (switch `/Game/member/Okajima/state/PlayerBaseV1State` (`self.CurrentState`)
        (:`NewEnumerator0`
          (if (`/Game/member/Okajima/Garbage/bp/BP_GrabActorT1V1.Break` (cast `/Game/member/Okajima/Garbage/bp/BP_GrabActorT1V1` (`self.Grab Item`) :!pure true))
            (set `self.CurrentState` "NewEnumerator7")))
        (:`NewEnumerator1`
          (`self.Function Lock On`))
        (:`NewEnumerator3`
          (`self.Function GBReady`))
        (:`NewEnumerator4`
          (`self.Function GB`))
        (:`NewEnumerator6`
          (`self.Function GBEnd`))
        (:`NewEnumerator7`
          (`self.Grabbing`))))
    (:`then_1`
      (`KismetSystemLibrary.PrintString` (`KismetSystemLibrary.GetDisplayName` (`self.Grab Item`))))))

(event `InputAxisKey|MouseWheelAxis`
  (params (AxisValue :type "Float (single-precision)"))
  (set `self.PredictionScale` (`KismetMathLibrary.FClamp` (+ (* AxisValue 100.0) (`self.PredictionScale`)) 0.0 2000.0)))

(event `Grabbing`
  (`|ExecutionSequence`
    (:`then_0`
      (`/Engine/EditorBlueprintResources/StandardMacros.DoOnce` false
        (:`Completed`
          (`self.SetActorEnableCollision` (stale _grab_item) true)
          (`KismetSystemLibrary.PrintString` "Grab Item Collision Enabled!" true true (struct :`R` 1.0 :`G` 0.143594 :`A` 1.0)))))
    (:`then_1`
      (bind _grab_item (`self.Grab Item`)
        (:`then`
          (`self.K2_SetActorLocation` _grab_item (`SceneComponent.K2_GetComponentLocation` (`self.Sphere`)) false false)
          (`KismetSystemLibrary.PrintString` (`KismetStringLibrary.Conv_VectorToString` (`self.K2_GetActorLocation` _grab_item))))
        (:`else`)))))

(fn `Create Prediction Path`
  (locals (SplineLocation :type "Array of Vector Structure") (LocalIndex :type Integer))
  (bind _sphere (`self.Sphere`))
  (bind _returnvalue (`SplineComponent.GetNumberOfSplineSegments` (`self.Spline`)))
  (bind (_location _tangent) (`SplineComponent.GetLocationAndTangentAtSplinePoint` (`self.Spline`) (`local.LocalIndex`) "World"))
  (bind (_location_2 _tangent_2) (`SplineComponent.GetLocationAndTangentAtSplinePoint` (`self.Spline`) (+ (`local.LocalIndex`) 1) "World"))
  (`|ExecutionSequence`
    (:`then_0`
      (bind _output_get (set `self.Velocity` (* (`KismetMathLibrary.GetForwardVector` (`SceneComponent.K2_GetComponentRotation` _sphere)) (`self.PredictionScale`))))
      (bind (_outhit _outpathpositions _outlasttracedestination _returnvalue_2) (`GameplayStatics.Blueprint_PredictProjectilePath_ByTraceChannel` (`SceneComponent.K2_GetComponentLocation` _sphere) _output_get true 20.0 "ECC_WorldDynamic" false (`|MakeArray` self :!type "Actor Object Reference") "ForOneFrame" 1.0))
      (set `local.SplineLocation` _outpathpositions)
      (if _returnvalue_2
        (`self.SetActorHiddenInGame` (`self.PredictionEnd`) false)
        (`self.K2_SetActorLocation` (`self.PredictionEnd`) _outlasttracedestination false true)
        (else
          (`self.SetActorHiddenInGame` (`self.PredictionEnd`) true))))
    (:`then_1`
      (`self.Destroy Prediction Path`)
      (`SplineComponent.SetSplinePoints` (`self.Spline`) (`local.SplineLocation`) "World" true)
      (`KismetSystemLibrary.PrintString` (`KismetStringLibrary.Conv_IntToString` _returnvalue))
      (for _index (range _returnvalue)
        (set `local.LocalIndex` _index)
        (bind _returnvalue_3 (`AddComponent|NODE_AddSplineMeshComponent-0` :`bManualAttachment` true))
        (`KismetArrayLibrary.Array_Add` (`self.PredictonPathMeshes`) _returnvalue_3)
        (`SplineMeshComponent.SetStartAndEnd` _returnvalue_3 _location _tangent _location_2 _tangent_2 true)))))

(fn `Destroy Prediction Path`
  (for _array_element (`self.PredictonPathMeshes`)
    (`ActorComponent.K2_DestroyComponent` _array_element))
  (`KismetArrayLibrary.Array_Clear` (`self.PredictonPathMeshes`)))

(fn `Function GB`
  (`|ExecutionSequence`
    (:`then_0`
      (`self.Function Lock On`))
    (:`then_1`
      (if (`self.Pulling`)
        (`self.Setting GB Controller Input Value`)
        (switch `/Game/member/Okajima/state/GrabBaseV1State` (`/Game/member/Okajima/Garbage/bp/BP_GrabActorT1V1.CurrentState` (cast `/Game/member/Okajima/Garbage/bp/BP_GrabActorT1V1` (`self.Grab Item`) :!pure true))
          (:`NewEnumerator2`)
          (:`NewEnumerator3`
            (bind _degree (`self.Get Degree` (`self.InputControllerYValue`) (`self.InputControllerXValue`)))
            (if (`KismetMathLibrary.NearlyEqual_FloatFloat` (`self.PullingDegree`) _degree 15.0)
              (set `self.CorrectPulling` true)
              (set `self.NotCorrectPulling` false)
              (`self.K2_AddActorWorldOffset` (`self.Grab Item`) (`KismetMathLibrary.MakeVector` (* (`KismetMathLibrary.DegCos` _degree) 0.1) (* (`KismetMathLibrary.DegSin` _degree) 0.1)) false false)
              (`GameplayStatics.ApplyDamage` (`self.Grab Item`) (`self.AttackPower`))
              (else
                (set `self.CorrectPulling` false)
                (set `self.NotCorrectPulling` true)))))))))

(fn `Function GBEnd`
  (bind (_returnvalue_x _returnvalue_y) (`KismetMathLibrary.BreakVector` (`SceneComponent.K2_GetComponentLocation` (`self.CapsuleComponent`))))
  (bind (_returnvalue_x_2 _returnvalue_y_2 _returnvalue_z) (`KismetMathLibrary.BreakVector` (`SceneComponent.K2_GetComponentLocation` (`self.SpringArm`))))
  (if (< (`SpringArmComponent.TargetArmLength` (`self.SpringArm`)) 450.0)
    (set `SpringArmComponent.TargetArmLength` (+ (`SpringArmComponent.TargetArmLength` (`self.SpringArm`)) 10.0) (`self.SpringArm`))
    (else
      (set `SpringArmComponent.TargetArmLength` 450.0 (`self.SpringArm`))
      (set `self.CurrentState` "NewEnumerator0")
      (`SceneComponent.K2_SetWorldLocation` (`self.SpringArm`) (`KismetMathLibrary.MakeVector` _returnvalue_x _returnvalue_y _returnvalue_z) false false)
      (set `self.MovingSpringArmLocationX` 0.0)
      (set `self.MovingSpringArmLocationY` 0.0))))

(fn `Function GBReady`
  (bind (_returnvalue_x _returnvalue_y) (`KismetMathLibrary.BreakVector` (`self.K2_GetActorLocation`)))
  (bind (_returnvalue_x_2 _returnvalue_y_2 _returnvalue_z) (`KismetMathLibrary.BreakVector` (`SceneComponent.K2_GetComponentLocation` (`self.SpringArm`))))
  (bind (_returnvalue_x_3 _returnvalue_y_3) (`KismetMathLibrary.BreakVector` (`self.K2_GetActorLocation` (`|GetArrayItem` (`self.Grab Items`) (`self.LockOnIndex`)))))
  (bind _returnvalue (`KismetMathLibrary.DegAtan2` (- _returnvalue_x_3 _returnvalue_x) (- _returnvalue_y_3 _returnvalue_y)))
  (bind _returnvalue_2 (/ (`KismetMathLibrary.Vector_Distance2D` (`self.K2_GetActorLocation` (`|GetArrayItem` (`self.Grab Items`) (`self.LockOnIndex`))) (`self.K2_GetActorLocation`)) 2.0))
  (bind _returnvalue_3 (+ _returnvalue_x_2 (* (`KismetMathLibrary.DegSin` _returnvalue) _returnvalue_2)))
  (bind _returnvalue_4 (+ _returnvalue_y_2 (* (`KismetMathLibrary.DegCos` _returnvalue) _returnvalue_2)))
  (if (> (`SpringArmComponent.TargetArmLength` (`self.SpringArm`)) (`self.ZoomUpCameraLength`))
    (set `SpringArmComponent.TargetArmLength` (- (`SpringArmComponent.TargetArmLength` (`self.SpringArm`)) 5.0) (`self.SpringArm`))
    (else
      (set `self.CurrentState` "NewEnumerator4")
      (set `self.MovingSpringArmLocationX` _returnvalue_3)
      (set `self.MovingSpringArmLocationY` _returnvalue_4)
      (`SceneComponent.K2_SetWorldLocation` (`self.SpringArm`) (`KismetMathLibrary.MakeVector` _returnvalue_3 _returnvalue_4 _returnvalue_z) false false))))

(fn `Function GReady`
  (bind (_returnvalue_x _returnvalue_y) (`KismetMathLibrary.BreakVector` (`SceneComponent.K2_GetComponentLocation` (`self.CapsuleComponent`))))
  (bind (_returnvalue_x_2 _returnvalue_y_2 _returnvalue_z) (`KismetMathLibrary.BreakVector` (`SceneComponent.K2_GetComponentLocation` (`self.SpringArm`))))
  (if (< (`SpringArmComponent.TargetArmLength` (`self.SpringArm`)) 450.0)
    (set `SpringArmComponent.TargetArmLength` (+ (`SpringArmComponent.TargetArmLength` (`self.SpringArm`)) 10.0) (`self.SpringArm`))
    (else
      (set `SpringArmComponent.TargetArmLength` 450.0 (`self.SpringArm`))
      (set `self.CurrentState` "NewEnumerator7")
      (`SceneComponent.K2_SetWorldLocation` (`self.SpringArm`) (`KismetMathLibrary.MakeVector` _returnvalue_x _returnvalue_y _returnvalue_z) false false)
      (set `self.MovingSpringArmLocationX` 0.0)
      (set `self.MovingSpringArmLocationY` 0.0))))

(fn `Function Lock On`
  (`SceneComponent.K2_SetWorldRotation` (`self.Mesh`) (`KismetMathLibrary.MakeRotator` (.roll (`KismetMathLibrary.FindLookAtRotation` (`self.K2_GetActorLocation`) (`self.K2_GetActorLocation` (`|GetArrayItem` (`self.Grab Items`) (`self.LockOnIndex`))))) (.pitch (`KismetMathLibrary.FindLookAtRotation` (`self.K2_GetActorLocation`) (`self.K2_GetActorLocation` (`|GetArrayItem` (`self.Grab Items`) (`self.LockOnIndex`))))) (+ (.yaw (`KismetMathLibrary.FindLookAtRotation` (`self.K2_GetActorLocation`) (`self.K2_GetActorLocation` (`|GetArrayItem` (`self.Grab Items`) (`self.LockOnIndex`))))) -90.0)) false false))

(fn `Get Degree`
  (params (X :type "Float (double-precision)") (Y :type "Float (double-precision)"))
  (returns (Degree :type "Float (double-precision)"))
  (return (/ (* (`KismetMathLibrary.Atan2` (- Y 0.0) (- X 0.0)) 180.0) 3.14)))

(fn `Setting GB Controller Input Value`
  (bind _asbp_grab_actor_t1v1 (cast `/Game/member/Okajima/Garbage/bp/BP_GrabActorT1V1` (`self.Grab Item`) :!pure true))
  (bind _returnvalue (+ (`self.PullingDegree`) 180.0))
  (bind _degree (`self.Get Degree` (`/Game/member/Okajima/Garbage/bp/BP_GrabActorT1V1.PullingYValue` _asbp_grab_actor_t1v1) (`/Game/member/Okajima/Garbage/bp/BP_GrabActorT1V1.PullingXValue` _asbp_grab_actor_t1v1)))
  (set `self.PullingDegree` _degree)
  (if (> _returnvalue 180.0)
    (set `self.PullingDegree` (- _returnvalue 360.0))
    (else
      (set `self.PullingDegree` _returnvalue))))

(fn `UserConstructionScript`)