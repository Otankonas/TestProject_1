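; Grab-target enemy actor that fights the player through a tug-of-war, with Battle, Pulling, Throw and Break states driven from Tick.
; In Battle it faces the player, updates balance gauges and breaks at zero, picks a random cardinal escape direction with slow motion and a widget arrow, then moves, spawning afterimages.
; A Pulling event restores time, and the DamagePulling timeline lerps it back to its start point.
; Throw steps it along stored path points each tick.
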(event `self.ReceiveTick`
  (params (DeltaSeconds :type "Float (single-precision)"))
  (`parent.ReceiveTick` DeltaSeconds)
  (switch `/Game/member/Okajima/state/GBaseV2State` (`self.Current State`)
    (:`NewEnumerator1`
      (`self.Battle`))
    (:`NewEnumerator3`
      (`self.Throw`))
    (:`NewEnumerator4`
      (`self.Pulling`))))

(event `Event Pulling`
  (switch `/Game/member/Okajima/state/GBaseV2State` (`self.Current State`)
    (:`NewEnumerator1`
      (set `self.Current State` "NewEnumerator4")
      (`KismetArrayLibrary.Array_Set` (`self.Pulling Direction`) 0 -100.0)
      (`KismetArrayLibrary.Array_Set` (`self.Pulling Direction`) 1 -100.0)
      (set `self.Pulling Location` (`self.K2_GetActorLocation`))
      (`GameplayStatics.SetGlobalTimeDilation` 1.0))))

(fn `Battle`
  (`|ExecutionSequence`
    (:`then_0`
      (`self.Recovery Gauge`))
    (:`then_1`
      (`self.Damage Gauge`)
      (if (`KismetMathLibrary.NearlyEqual_FloatFloat` (`self.Current Balance Point`))
        (`GameplayStatics.SetGlobalTimeDilation` 1.0)
        (set `self.Balance Break` true)
        (set `self.Current State` "NewEnumerator2")
        (`self.SetActorEnableCollision` false)
        (`/Game/member/Okajima/wbp/WBP_SampleDirectionV1.is not Show` (`self.As WBP Sample Direction V1`))))
    (:`then_2`
      (`self.Lock On`))
    (:`then_3`
      (if (`self.Attack`)
        (`self.Movement`)
        (else
          (`self.Setting Pulling Direction`)
          (`KismetSystemLibrary.PrintString` "Setting Pulling Direction Value!" true true (struct :`R` 1.0 :`G` 0.02448 :`A` 1.0))
          (set `self.Attack` true)
          (set `self.Current Location` (`self.K2_GetActorLocation`))
          (`GameplayStatics.SetGlobalTimeDilation` 0.05)
          (`/Game/member/Okajima/wbp/WBP_SampleDirectionV1.is SHow` (`self.As WBP Sample Direction V1`))
          (`|ExecutionSequence`
            (:`then_0`
              (if (`KismetMathLibrary.NearlyEqual_FloatFloat` (`|GetArrayItem` (`self.Pulling Direction`)) 1.0)
                (`/Game/member/Okajima/wbp/WBP_SampleDirectionV1.Arrow Right` (`self.As WBP Sample Direction V1`))))
            (:`then_1`
              (if (`KismetMathLibrary.NearlyEqual_FloatFloat` (`|GetArrayItem` (`self.Pulling Direction`)) -1.0)
                (`/Game/member/Okajima/wbp/WBP_SampleDirectionV1.Arrow Left` (`self.As WBP Sample Direction V1`))))
            (:`then_2`
              (if (`KismetMathLibrary.NearlyEqual_FloatFloat` (`|GetArrayItem` (`self.Pulling Direction`) 1) 1.0)
                (`/Game/member/Okajima/wbp/WBP_SampleDirectionV1.Arrow Top` (`self.As WBP Sample Direction V1`))))
            (:`then_3`
              (if (`KismetMathLibrary.NearlyEqual_FloatFloat` (`|GetArrayItem` (`self.Pulling Direction`) 1) -1.0)
                (`/Game/member/Okajima/wbp/WBP_SampleDirectionV1.Arrow Down` (`self.As WBP Sample Direction V1`))))))))))

(fn `Lock On`
  (`SceneComponent.K2_SetWorldRotation` (`self.Mesh`) (`KismetMathLibrary.MakeRotator` (.roll (`KismetMathLibrary.FindLookAtRotation` (`self.K2_GetActorLocation`) (`self.K2_GetActorLocation` (`self.As BP Player Base V2`)))) (.pitch (`KismetMathLibrary.FindLookAtRotation` (`self.K2_GetActorLocation`) (`self.K2_GetActorLocation` (`self.As BP Player Base V2`)))) (+ (.yaw (`KismetMathLibrary.FindLookAtRotation` (`self.K2_GetActorLocation`) (`self.K2_GetActorLocation` (`self.As BP Player Base V2`)))) -90.0)) false false))

(fn `Movement`
  (bind (_returnvalue_location _returnvalue_rotation _returnvalue_scale) (`KismetMathLibrary.BreakTransform` (`self.GetTransform`)))
  (bind (_returnvalue_roll _returnvalue_pitch _returnvalue_yaw) (`KismetMathLibrary.BreakRotator` (`SceneComponent.K2_GetComponentRotation` (`self.Mesh`))))
  (`self.AddMovementInput` (0.0 1.0 0.0) (`|GetArrayItem` (`self.Pulling Direction`)))
  (`self.AddMovementInput` (1.0 0.0 0.0) (`|GetArrayItem` (`self.Pulling Direction`) 1))
  (`|SpawnActorFromClass` "/Game/member/Okajima/Garbage/bp/BP_GrabActorT1V1AfterEffect.BP_GrabActorT1V1AfterEffect_C" (`KismetMathLibrary.MakeTransform` _returnvalue_location (`KismetMathLibrary.MakeRotator` _returnvalue_roll _returnvalue_pitch (+ _returnvalue_yaw 90.0)) _returnvalue_scale) "Undefined" "OverrideRootScale" null (struct) null)
  (if (> (`KismetMathLibrary.Vector_Distance` (`self.Current Location`) (`self.K2_GetActorLocation`)) 10.0)
    _))

(fn `Pulling`
  (if (not (`TimelineComponent.IsPlaying` (`self.Damage Pulling`)))
    (`TimelineComponent.PlayFromStart` (`self.Damage Pulling`))))

(fn `Setting Pulling Direction`
  (if (`KismetMathLibrary.RandomBool`)
    (if (`KismetMathLibrary.RandomBool`)
      (`KismetArrayLibrary.Array_Set` (`self.Pulling Direction`) 0 1.0)
      (`KismetArrayLibrary.Array_Set` (`self.Pulling Direction`) 1)
      (else
        (`KismetArrayLibrary.Array_Set` (`self.Pulling Direction`) 0 -1.0)
        (`KismetArrayLibrary.Array_Set` (`self.Pulling Direction`) 1)))
    (elif (`KismetMathLibrary.RandomBool`)
      (`KismetArrayLibrary.Array_Set` (`self.Pulling Direction`))
      (`KismetArrayLibrary.Array_Set` (`self.Pulling Direction`) 1 1.0)
      (else
        (`KismetArrayLibrary.Array_Set` (`self.Pulling Direction`))
        (`KismetArrayLibrary.Array_Set` (`self.Pulling Direction`) 1 -1.0))))
  (`KismetSystemLibrary.PrintString` "Pulling Direction X" true true (struct :`R` 1.0 :`B` 0.805182 :`A` 1.0))
  (`KismetSystemLibrary.PrintString` (`KismetStringLibrary.Conv_DoubleToString` (`|GetArrayItem` (`self.Pulling Direction`))))
  (`KismetSystemLibrary.PrintString` "Pulling Direction Y" true true (struct :`R` 1.0 :`B` 0.805182 :`A` 1.0))
  (`KismetSystemLibrary.PrintString` (`KismetStringLibrary.Conv_DoubleToString` (`|GetArrayItem` (`self.Pulling Direction`) 1))))

(fn `Throw`
  (if (< (`self.ThrowPath Index`) (- (`KismetArrayLibrary.Array_Length` (`self.ThrowPath Location`)) 1))
    (`self.K2_SetActorLocation` (`|GetArrayItem` (`self.ThrowPath Location`) (`self.ThrowPath Index`)))
    (`/Engine/EditorBlueprintResources/StandardMacros.IncrementInt` (`self.ThrowPath Index`))
    (else
      (set `self.Current State` "NewEnumerator0")
      (set `self.ThrowPath Index` 0))))

(fn `UserConstructionScript`
  (`parent.UserConstructionScript`))