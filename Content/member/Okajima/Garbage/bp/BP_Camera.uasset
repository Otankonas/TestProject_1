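; Side-scrolling camera actor that becomes the player's view target on BeginPlay and follows the player pawn.
; Each tick it tracks the pawn's X, updating height only while IsJumpMove is set and otherwise holding the stored LocationZ.
; When IsBoss is set, it instead lerps from CameraPos to BossPos by incrementing alpha per tick, unless CameraStop is set.
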(event `self.ReceiveBeginPlay`
  (bind _returnvalue (`GameplayStatics.GetPlayerController` 0))
  ;[1 1 1] 初期配置
  (`PlayerController.SetViewTargetWithBlend` _returnvalue self 0.0 "VTBlend_Linear" 0.0 false)
  (`self.SetLocation2D` (`self.K2_GetActorLocation` _returnvalue))
  (`self.K2_SetActorRotation` (`KismetMathLibrary.MakeRotator` 0.0)))

(event `self.ReceiveTick`
  (params (DeltaSeconds :type "Float (single-precision)"))
  (bind _returnvalue (`self.K2_GetActorLocation` (`GameplayStatics.GetPlayerPawn` 0)))
  (if (`self.IsBoss`)
    ;[1 1 1] ボス部屋
    (if (not (`self.CameraStop`))
      (`self.K2_SetActorLocation` (`KismetMathLibrary.VLerp` (`self.CameraPos`) (`self.BossPos`) (`self.LerpTime`)))
      (if (< (`self.LerpTime`) 1.0)
        (set `self.LerpTime` (+ (`self.LerpTime`) 0.05))))
    (elif (`self.IsJumpMove`)
      (`self.SetLocation2D` _returnvalue)
      (else
        (`self.SetLocation` _returnvalue)))))

(fn `SetLocation`
  (params (NewParam :type "Vector Structure"))
  (`self.K2_SetActorLocation` (`KismetMathLibrary.MakeVector` NewParam_X 0.0 (`self.LocationZ`)) true))

(fn `SetLocation2D`
  (params (self2 :type "Vector Structure"))
  (bind _output_get (set `self.LocationZ` self2_Z))
  (`self.K2_SetActorLocation` (`KismetMathLibrary.MakeVector` self2_X 0.0 _output_get) true))

(fn `UserConstructionScript`)