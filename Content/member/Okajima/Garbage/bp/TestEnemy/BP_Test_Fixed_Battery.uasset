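; Test fixed battery enemy that fires a shell when the player pawn enters its line of sight.
; Each tick it line-traces from the firing point along a world axis chosen by the IsTop and IsLeft flags, which also orient the box in the construction script.
; On the first player hit it spawns a scaled-down shell carrying those flags; IsFire is never reset, so it fires only once.
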(event `self.ReceiveTick`
  (params (DeltaSeconds :type "Float (single-precision)"))
  (bind (_start_pos _end_pos) (`self.Get LineTrace Pos`))
  (bind _outhit (`KismetSystemLibrary.LineTraceSingle` _start_pos _end_pos "TraceTypeQuery1" false (`self.Ignore Actors`)))
  (if (== (`.HitActor` (`GameplayStatics.BreakHitResult` _outhit)) (`GameplayStatics.GetPlayerPawn` 0))
    (if (not (`self.isFire`))
      (set `self.isFire` true)
      (`self.Fire`))))

(event `Charge`)

(event `Fire`
  (bind (_returnvalue_location _returnvalue_rotation) (`KismetMathLibrary.BreakTransform` (`SceneComponent.K2_GetComponentToWorld` (`self.Firing Point`))))
  (`|SpawnActorFromClass` "/Game/member/Okajima/Garbage/bp/TestEnemy/BP_Test_Shell_Of_A_Battery.BP_Test_Shell_Of_A_Battery_C" (`KismetMathLibrary.MakeTransform` _returnvalue_location _returnvalue_rotation (0.25 0.25 0.25)) "Undefined" "OverrideRootScale" null (`self.isLeft`) (`self.isTop`) null))

(fn `UserConstructionScript`
  (if (`self.isTop`)
    (`SceneComponent.K2_SetWorldRotation` (`self.Box`) (struct :`Yaw` 90.0) false false)
    (elif (`self.isLeft`)
      (`SceneComponent.K2_SetWorldRotation` (`self.Box`) (struct :`Yaw` 180.0) false false)
      (else
        (`SceneComponent.K2_SetWorldRotation` :`self` (`self.Box`))))))