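; Test projectile actor, named as the shell of an enemy battery, that flies along one of three fixed world directions.
; On BeginPlay, the IsTop and IsLeft flags pick a hard-coded root rotation and matching ProjectileMovement velocity, with IsTop taking priority over left or right.
; It has no active overlap, tick or hit logic.
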(event `self.ReceiveBeginPlay`
  (if (`self.isTop`)
    (`SceneComponent.K2_SetWorldRotation` :`self` (`self.DefaultSceneRoot`))
    (set `MovementComponent.Velocity` (-100.0 0.0 0.0) (`self.ProjectileMovement`))
    (elif (`self.isLeft`)
      (`SceneComponent.K2_SetWorldRotation` (`self.DefaultSceneRoot`) (struct :`Yaw` 90.0) false false)
      (set `MovementComponent.Velocity` (0.0 -100.0 0.0) (`self.ProjectileMovement`))
      (else
        (`SceneComponent.K2_SetWorldRotation` (`self.DefaultSceneRoot`) (struct :`Yaw` -90.0) false false)
        (set `MovementComponent.Velocity` (0.0 100.0 0.0) (`self.ProjectileMovement`))))))

(fn `UserConstructionScript`)