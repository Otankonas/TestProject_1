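; Test enemy that takes damage, shows HP on a widget-component gauge and runs a frame-counted action state machine.
; Tick advances a frame counter, dispatches Attack, Avoid and FAILED handlers, and prints the state for debugging.
; Finished actions return to Idle and set a stop-operator countdown, which nothing here uses for gating.
; Attack switches unconditionally to FAILED partway through; Grabbed and Success have no per-frame handlers.
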(event `self.ReceiveBeginPlay`
  (`|ExecutionSequence`
    (:`then_0`
      (`self.Bind WBP`))
    (:`then_1`
      (set `self.Current State` "NewEnumerator0")
      (set `self.Chance Zone` true)
      (set `self.Anim Frame` 0)
      (set `self.Finish Anim Frame` 0)
      (set `self.Stop Operator Frame` 0))))

(event `Stop Operator`
  (params (`Delay Frame` :type Integer))
  (set `self.Stop Operator Frame` `Delay Frame`))

(event `self.ReceiveAnyDamage`
  (params (Damage :type "Float (single-precision)") (DamageType :type "DamageType Object Reference") (InstigatedBy :type "Controller Object Reference") (DamageCauser :type "Actor Object Reference"))
  (bind _output_get (set `self.HP` (`KismetMathLibrary.FMax` (- (`self.HP`) Damage))))
  (if (`KismetMathLibrary.NearlyEqual_FloatFloat` _output_get)
    (`/Game/member/Okajima/wbp/WBP_SampleGageV1.UpdateHealthProgress` (`self.HP Gage`) 0.0)
    (else
      (`/Game/member/Okajima/wbp/WBP_SampleGageV1.UpdateHealthProgress` (`self.HP Gage`) (/ (`self.HP`) (`self.MAXHP`))))))

(event `self.ReceiveTick`
  (params (DeltaSeconds :type "Float (single-precision)"))
  (bind _current_state (`self.Current State`))
  (bind _anim_frame (`self.Anim Frame`))
  (`self.execute Stop Operator`)
  (`|ExecutionSequence`
    (:`then_0`
      (`self.Update All State` _anim_frame _current_state)
      (`/Engine/EditorBlueprintResources/StandardMacros.IncrementInt` _anim_frame))
    (:`then_1`
      (`KismetSystemLibrary.PrintString` (`|GetEnumeratorNameAsString` _current_state)))))

(event `Attack Event`
  (params (`Current Frame` :type Integer))
  (`self.is Animation Now` `Current Frame`
    (:`then`
      (`self.set Anim Default` 30))
    (:`else`
      (if (>= `Current Frame` 14)
        (`self.Set Current State` "NewEnumerator6")))))

(event `FAILED Event`
  (params (`Current Frame` :type Integer))
  (`self.is Animation Now` `Current Frame`
    (:`then`
      (`self.set Anim Default` 30))))

(event `Avoid Event`
  (params (`Current Frame` :type Integer))
  (`self.is Animation Now` `Current Frame`
    (:`then`
      (`self.set Anim Default` 30))))

(fn `Bind WBP`
  (bind _aswbp_sample_gage_v1 (cast `/Game/member/Okajima/wbp/WBP_SampleGageV1` (`WidgetComponent.GetUserWidgetObject` (`self.Widget`))))
  (bind _output_get (set `self.HP Gage` _aswbp_sample_gage_v1))
  (`/Game/member/Okajima/wbp/WBP_SampleGageV1.UpdateHealthProgress` _output_get (/ (`self.HP`) (`self.MAXHP`))))

(fn `Set Current State`
  (params (`Next State` :type "/Game/member/Okajima/EnemySource/TestEnemy/BP_TestEnemyAnimState Enum" :default "NewEnumerator0"))
  (set `self.Current State` `Next State`)
  (set `self.Anim Frame` 0)
  (switch `/Game/member/Okajima/EnemySource/TestEnemy/BP_TestEnemyAnimState` `Next State`
    (:`NewEnumerator0`
      (set `self.Finish Anim Frame` 0))
    (:`NewEnumerator1`
      (set `self.Finish Anim Frame` 50))
    (:`NewEnumerator2`
      (set `self.Finish Anim Frame` 26))
    (:`NewEnumerator6`
      (set `self.Finish Anim Frame` 36))
    (:`NewEnumerator7`
      (set `self.Finish Anim Frame` 0))
    (:`NewEnumerator8`
      (set `self.Finish Anim Frame` 48))))

(fn `Update All State`
  (params (`Current Frame` :type Integer) (`Current State` :type "/Game/member/Okajima/EnemySource/TestEnemy/BP_TestEnemyAnimState Enum" :default "NewEnumerator0"))
  (switch `/Game/member/Okajima/EnemySource/TestEnemy/BP_TestEnemyAnimState` `Current State`
    (:`NewEnumerator1`
      (`self.Attack Event` `Current Frame`))
    (:`NewEnumerator2`
      (`self.Avoid Event` `Current Frame`))
    (:`NewEnumerator6`
      (`self.FAILED Event` `Current Frame`))))

(fn `UserConstructionScript`
  (set `self.HP` (`self.MAXHP`)))