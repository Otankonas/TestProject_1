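; Test enemy A character that reads Attack, Sensed and target from its AIC_EnemyA blackboard each Tick, unless held or frozen by a hit-stop-style frame counter.
; While unsensed it jitters by random swept offsets.
; Attack triggers a once-gated pseudo jump, with timelines lerping it upward then toward the player's position, and a delay clears the flag.
; State and animation-frame helpers exist, but Tick does not use them.
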(event `self.ReceiveBeginPlay`
  (`parent.ReceiveBeginPlay`)
  (`|ExecutionSequence`
    (:`then_0`
      (`self.Bind AIC BB`))
    (:`then_1`
      (set `self.Current State` "NewEnumerator0"))))

(event `Stop Operator`
  (params (`Delay Frame` :type Integer))
  ;[0 0.5834 1] Set Rigidity
  (set `self.Stop Operator Frame` `Delay Frame`))

(event `self.ReceiveTick`
  (params (DeltaSeconds :type "Float (single-precision)"))
  (bind _returnvalue (`self.K2_GetActorLocation`))
  (`parent.ReceiveTick` DeltaSeconds)
  (`self.Execute Stop Operator`
    (:`then`
      (`self.is Hold`
        (:`else`
          (`|ExecutionSequence`
            (:`then_0`
              (`self.Update AIC BB`))
            (:`then_1`
              (`self.is Sensed`
                (:`else`
                  (bind (_sweephitresult _returnvalue_2) (`self.K2_SetActorLocation` (+ (`KismetMathLibrary.RandomUnitVectorInConeInRadians` _returnvalue 250.0) _returnvalue) true))
                  (`KismetSystemLibrary.PrintString` (`KismetStringLibrary.Conv_BoolToString` _returnvalue_2)))))
            (:`then_2`
              (`self.is Atk`
                (:`then`
                  (`/Engine/EditorBlueprintResources/StandardMacros.DoOnce` false :!label _label
                    (:`Completed`
                      (`KismetArrayLibrary.Array_Set` (`self.Target Location`) 0 (`self.K2_GetActorLocation`))
                      (`KismetArrayLibrary.Array_Set` (`self.Target Location`) 1 (+ (`self.K2_GetActorLocation`) (0.0 0.0 300.0)))
                      (`TimelineComponent.PlayFromStart` (`self.Pseudo Jump To Z`)))))
                (:`else`
                  (goto _label :!via `Reset`))))
            (:`then_3`
              (`KismetSystemLibrary.Delay` 5.0)
              (`self.Set Atk` false))))))))

(fn `Bind AIC BB`
  (bind _returnvalue (`self.GetController`))
  (bind _asaic_enemy_a (cast `/Game/member/Okajima/EnemySource/SampleAITest/AIC_EnemyA` _returnvalue))
  (set `self.AICtl` _asaic_enemy_a)
  (set `self.AIBB` (`AIBlueprintHelperLibrary.GetBlackboard` _returnvalue)))

(fn `Set Current State`
  (params (`Next State` :type "/Game/member/Okajima/EnemySource/akr/BP_EnemyA_TestV1State Enum" :default "NewEnumerator0"))
  (set `self.Current State` `Next State`)
  (set `self.Anim Frame` 0)
  (switch `/Game/member/Okajima/EnemySource/akr/BP_EnemyA_TestV1State` (`self.Current State`)
    (:`NewEnumerator0`
      (set `self.Finish Anim Frame` 0 :!label _label))
    (:`NewEnumerator1`
      (goto _label))
    (:`NewEnumerator2`
      (set `self.Finish Anim Frame` 60))
    (:`NewEnumerator3`
      (set `self.Finish Anim Frame` 45))
    (:`NewEnumerator4`
      (set `self.Finish Anim Frame` 92))))

(fn `Update AIC BB`
  (set `self.Attack` (`BlackboardComponent.GetValueAsBool` (`self.AIBB`) "Attack"))
  (bind _output_get (set `self.Sensed` (`BlackboardComponent.GetValueAsBool` (`self.AIBB`) "Sensed")))
  (set `self.Target` (`BlackboardComponent.GetValueAsObject` (`self.AIBB`) "TargetActor")))

(fn `UserConstructionScript`
  (`parent.UserConstructionScript`)
  (`KismetArrayLibrary.Array_Set` (`self.Target Location`) 3 (`self.K2_GetActorLocation`)))