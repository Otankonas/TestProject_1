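; BP_DummyEnemy is a dummy enemy Blueprint that sketches a frame-counted state machine with Idle, Move, Attack and Gotcha states.
; It starts in Idle, and Tick passes the state and frame counter to UpdateAllState before incrementing the counter.
; SetCurrentState resets the counter and sets each state's finish frame, nonzero only for Attack.
; It is a skeleton: the update switch has no branches and the state events are empty.
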(event `self.ReceiveBeginPlay`
  (`parent.ReceiveBeginPlay`)
  (`|ExecutionSequence`
    (:`then_0`
      (set `self.Anim Frame Count` 0)
      (set `self.Finish Anim Frame Count` 0)
      (set `self.Current State` "NewEnumerator0"))))

(event `self.ReceiveTick`
  (params (DeltaSeconds :type "Float (single-precision)"))
  (bind _anim_frame_count (`self.Anim Frame Count`))
  (`parent.ReceiveTick` DeltaSeconds)
  (`|ExecutionSequence`
    (:`then_0`
      (`self.Update All State` _anim_frame_count (`self.Current State`))
      (`/Engine/EditorBlueprintResources/StandardMacros.IncrementInt` _anim_frame_count))))

(event `Idle Event`)

(event `Move Event`)

(event `Attack Event`)

(event `Gotcha Event`)

(fn `Set Current State`
  (params (`Next State` :type "/Game/member/Okajima/EnemySource/DummyEnemy/BP_DummyEnemyAnimState Enum" :default "NewEnumerator0"))
  (set `self.Current State` `Next State`)
  (set `self.Anim Frame Count` 0)
  (switch `/Game/member/Okajima/EnemySource/DummyEnemy/BP_DummyEnemyAnimState` `Next State`
    (:`NewEnumerator0`
      (set `self.Finish Anim Frame Count` 0))
    (:`NewEnumerator1`
      (set `self.Finish Anim Frame Count` 0))
    (:`NewEnumerator2`
      (set `self.Finish Anim Frame Count` 50))
    (:`NewEnumerator3`
      (set `self.Finish Anim Frame Count` 0))))

(fn `Update All State`
  (params (`Current Frame` :type Integer) (`Current State` :type "/Game/member/Okajima/EnemySource/DummyEnemy/BP_DummyEnemyAnimState Enum" :default "NewEnumerator0"))
  (switch `/Game/member/Okajima/EnemySource/DummyEnemy/BP_DummyEnemyAnimState` `Current State`))

(fn `UserConstructionScript`
  (`parent.UserConstructionScript`))